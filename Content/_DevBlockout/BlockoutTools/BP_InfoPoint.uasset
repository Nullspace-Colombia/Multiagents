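; BP_InfoPoint is a blockout tool info marker that reveals its text display when a Character enters its capsule.
; On overlap it plays an attached sound and, if no animation is running, yaws the Rotatable component toward the Character.
; A timeline with sinusoidal ease-out moves and rotates the mesh and animates scale, reversing when an overlap ends.
; Actor tick is disabled in the construction script.
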(event OnComponentBeginOverlap(Capsule)
  (params (OverlappedComponent :type Primitive%20Component%20Object%20Reference) (OtherActor :type Actor%20Object%20Reference) (OtherComp :type Primitive%20Component%20Object%20Reference) (OtherBodyIndex :type Integer) (bFromSweep :type Boolean) (SweepResult :type Hit%20Result%20Structure%20%28by%20ref%29))
  (Utilities|Casting|CastToCharacter OtherActor)
  (Audio|SpawnSoundAttached 0 (Variables|Default|GetRotatable) "None" "0, 0, 0" "0, 0, 0" "KeepRelativeOffset" false 1.0 1.0 0.0 0 0) ; Interaction sound
  (if (not (Components|Activation|IsActive)) ; Run animation only if previous animation has finished
    (Transformation|SetWorldRotation (Variables|Default|GetRotatable) (Math|Rotator|MakeRotator 0.0 0.0 (.yaw (Math|Rotator|FindLookatRotation (Transformation|GetWorldLocation) (Transformation|GetActorLocation OtherActor)))) false false) ; Align text to Pawn camera
    (bind _newtrack_0 (Timeline|TimeLine_Linear PlayFromStart) ; Reverse animation on end collision
      (:Update
        (Variables|Default|SetAnimationProgress _newtrack_0)
        ;[0.1098 0.6667 0.5373] Animate Static meshes
        (Transformation|SetRelativeLocationAndRotation (Variables|Default|GetStaticMesh) (Math|Interpolation|Ease "SinusoidalOut" (Variables|Default|GetAnimationProgress) "0.000000,0.000000,30.000000" (Math|Vector|MakeVector 0.0 -3e+01 1.2e+02)) (Math|Interpolation|Ease :Function "SinusoidalOut" :Alpha (Variables|Default|GetAnimationProgress) :B (Math|Rotator|MakeRotator 9e+01 0.0 0.0)) false false)
        (Transformation|SetRelativeScale3D (Math|Interpolation|Ease :Function "SinusoidalOut" :Alpha (Variables|Default|GetAnimationProgress) :B "1.000000,1.000000,1.000000"))))))

(event OnComponentEndOverlap(Capsule)
  (params (OverlappedComponent :type Primitive%20Component%20Object%20Reference) (OtherActor :type Actor%20Object%20Reference) (OtherComp :type Primitive%20Component%20Object%20Reference) (OtherBodyIndex :type Integer))
  (bind _newtrack_0 (Timeline|TimeLine_Linear Reverse) ; Reverse animation on end collision
    (:Update
      (Variables|Default|SetAnimationProgress _newtrack_0)
      ;[0.1098 0.6667 0.5373] Animate Static meshes
      (Transformation|SetRelativeLocationAndRotation (Variables|Default|GetStaticMesh) (Math|Interpolation|Ease "SinusoidalOut" (Variables|Default|GetAnimationProgress) "0.000000,0.000000,30.000000" (Math|Vector|MakeVector 0.0 -3e+01 1.2e+02)) (Math|Interpolation|Ease :Function "SinusoidalOut" :Alpha (Variables|Default|GetAnimationProgress) :B (Math|Rotator|MakeRotator 9e+01 0.0 0.0)) false false)
      (Transformation|SetRelativeScale3D (Math|Interpolation|Ease :Function "SinusoidalOut" :Alpha (Variables|Default|GetAnimationProgress) :B "1.000000,1.000000,1.000000")))))

(fn ConstructionScript
  (Actor|Tick|SetActorTickEnabled false) ; We don't want this Actor to tick
)