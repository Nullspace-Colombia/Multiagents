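; Test Blueprint for a network client that starts a connection to a local server on BeginPlay.
; The SyncData_2 graph binds a data-reception delegate that converts incoming data into Actions and opens a gate.
; Its Hop event conducts the connection and, if connected, enters that gate, whose exit leads nowhere.
; SyncData_2 sits unwired in the event graph, so the sync logic never runs.
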(event Custom|StartConnection
  (Class|Pole|StartClient "127.0.0.1" 10011))

(event EventBeginPlay
  (CallFunction|StartConnection))

(event Collision|EventActorBeginOverlap
  (params (OtherActor :type Actor%20Object%20Reference)))

(event EventTick
  (params (DeltaSeconds :type Float%20%28single-precision%29)))

(fn ConstructionScript)

(event Custom|Open_Gate
  (Utilities|FlowControl|Gate false) ; enters at Open
)

(event Custom|Close_Gate
  (Utilities|FlowControl|Gate false) ; enters at Close
)

(event Custom|Hop
  (Class|Pole|ConductConnection)
  (if (Variables|Default|Getconnected)
    (Utilities|FlowControl|Gate false)))

(event Custom|OnDataReceptionDelegate_Event_0
  (params (Arr :type Array%20of%20Bytes))
  (bind _returnvalue (Class|Pole|GetAction Arr))
  (Variables|Default|SetActions _returnvalue)
  (CallFunction|OpenGate))