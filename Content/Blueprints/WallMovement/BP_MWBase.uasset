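; Base reinforcement-learning agent for a task of moving a pushbar to a goal, exposing state, reward, done and reset functions.
; Step counts frames and maps a discrete action to movement along the actor's right or forward axis.
; Observations combine XY location with four world-axis line traces, while rewards favor goal hits, bar contact and shrinking distances.
; Episodes end on goal hit or frame limit, and reset teleports only the pushbar.
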(event OnActorHit(pushbar)
  (params (SelfActor :type Actor%20Object%20Reference) (OtherActor :type Actor%20Object%20Reference) (NormalImpulse :type Vector :default "0, 0, 0") (Hit :type Hit%20Result%20Structure%20%28by%20ref%29))
  (if (== OtherActor (Variables|Default|Getgoal))
    (Variables|Default|SetDone (or (Variables|Default|GetDone) true))
    (Variables|Default|Settouch_goal true)
    (Development|PrintString "touched goal")
    (else
      (Variables|Default|SetDone (or (Variables|Default|GetDone) false))
      (if (== OtherActor self)
        (Variables|Default|Settouched true)
        (Development|PrintString "touched")
        (Development|PrintString (Utilities|GetDisplayName OtherActor))))))

(event Custom|CustomEvent
  (params (ID :type Float%20%28double-precision%29))
  (Variables|Default|SetID ID))

(event EventMove
  (params (NewParam :type Float%20%28double-precision%29))
  (bind _returnvalue (Transformation|GetActorForwardVector))
  (bind _returnvalue_2 (Transformation|GetActorRightVector))
  ;[1 1 1] movement
  (if (== NewParam 0.0)
    (Pawn|Input|AddMovementInput _returnvalue_2 1.0 false)
    (elif (== NewParam 1.0)
      (Pawn|Input|AddMovementInput _returnvalue_2 -1.0 false)
      (elif (== NewParam 2.0)
        (Pawn|Input|AddMovementInput _returnvalue 1.0 false)
        (elif (== NewParam 3.0)
          (Pawn|Input|AddMovementInput _returnvalue -1.0 false))))))

(event Collision|EventActorBeginOverlap
  (params (OtherActor :type Actor%20Object%20Reference)))

(event EventStep
  (params (Action :type Float%20%28double-precision%29))
  ;[1 1 1] Step
  (Math|Integer|IncrementInt (Variables|Default|GetCounter)
    (:%20%20
      (CallFunction|Move Action))))

(event EventBeginPlay)

(fn ConstructionScript
  (bind _returnvalue (Rendering|Material|CreateDynamicMaterialInstance (Variables|Default|GetCube) 0 0 "None" :!class /Script/Engine.PrimitiveComponent))
  (Rendering|Material|SetVectorParameterValue _returnvalue "Param" (Variables|Default|GetColor) :!class /Script/Engine.MaterialInstanceDynamic))

(fn GetAgentState
  (bind _returnvalue (Transformation|GetActorLocation))
  (bind _output_get (Variables|Default|Setobs (Utilities|Array|MakeArray (.x _returnvalue) (.y _returnvalue))))
  (bind _raytraces (|rayTracers)
    (:execute2
      (Utilities|Array|AppendArray _output_get _raytraces)
      (return (Variables|Default|Getobs)))))

(fn GetAgentReward
  (bind _returnvalue (Transformation|GetActorLocation))
  (bind _goal (Variables|Default|Getgoal))
  (bind _pushbar (Variables|Default|Getpushbar))
  (bind _returnvalue_2 (Transformation|GetActorLocation _goal))
  (bind _returnvalue_3 (Transformation|GetActorLocation _pushbar))
  (bind _returnvalue_4 (Math|Vector|Distance2D(Vector) (Math|Vector2D|MakeVector2D (.x _returnvalue_2) (.y _returnvalue_2)) (Math|Vector2D|MakeVector2D (.x _returnvalue_3) (.y _returnvalue_3))))
  (bind _returnvalue_5 (Math|Vector|Distance2D(Vector) (Math|Vector2D|MakeVector2D (.x _returnvalue_3) (.y _returnvalue_3)) (Math|Vector2D|MakeVector2D (.x _returnvalue) (.y _returnvalue))))
  (if (Variables|Default|Gettouch_goal)
    (Variables|Default|SetReward 1.0)
    (Variables|Default|Settouch_goal false)
    (elif (Variables|Default|Gettouched)
      (Variables|Default|Settouched false)
      (if (<= _returnvalue_4 (Variables|Default|Getprevious_distance_bar_goal))
        (Variables|Default|Setprevious_distance_bar_goal _returnvalue_4)
        (Variables|Default|SetReward 0.5)
        (else
          (Variables|Default|SetReward 0.2)))
      (elif (<= _returnvalue_5 (Variables|Default|Getprevious_distance_bar_agent))
        (Variables|Default|Setprevious_distance_bar_agent _returnvalue_5)
        (Variables|Default|SetReward 0.1)
        (else
          (Variables|Default|SetReward -0.1)))))
  (return (Variables|Default|GetReward)))

(fn IsAgentDone
  (Math|Integer|CompareInt (Variables|Default|GetCounter) (Variables|Default|GetMaxFrames)
    (:>
      (Variables|Default|SetDone (or (Variables|Default|GetDone) true) :!label _label)
      (Variables|Default|SetCounter 0))
    (:==
      (goto _label))
    (:<
      (Variables|Default|SetDone (or (Variables|Default|GetDone) false))))
  (return (Variables|Default|GetDone)))

(fn ResetAgent
  (Transformation|SetActorLocationAndRotation (Variables|Default|Getpushbar) "450.000000,1350.000000,50.000000" "0, 0, 0" false true)
  (return 0))

(fn OnRepPushbar)

(fn GetID
  (return 0))

(fn GetReward
  (bind _agentreward (CallFunction|GetAgentReward))
  (return _agentreward))

(fn GetSelfActor
  (return self))

(fn GetState
  (bind _pos (CallFunction|GetAgentState))
  (return _pos))

(fn IsDone
  (bind _isagentdone (CallFunction|IsAgentDone))
  (return _isagentdone))

(fn Reset
  (bind _newactor (CallFunction|ResetAgent))
  (Variables|Default|SetDone false)
  (return _newactor true))