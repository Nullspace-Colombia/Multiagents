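; PushBar_Arena is an arena actor that sets up two BP_MWBase agents for a wall-movement scenario.
; On BeginPlay it casts both child actors, caches them in an Agents array, then attaches each to the scene root at a fixed relative position.
; A failed cast only prints an error.
; Per-agent SetLimits calls derived from agent locations exist but are disconnected, so no movement bounds are applied here.
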(event EventBeginPlay
  (bind _asbp_mwbase (Utilities|Casting|CastToBP_MWBase (Variables|/Script/Engine.ChildActorComponent|GetChildActor (Variables|Default|GetBP_MWAgent1)))
    (:then
      (Variables|Default|SetAgent1 _asbp_mwbase)
      (Utilities|Array|Add (Variables|Default|GetAgents) 0)
      (bind _asbp_mwbase_2 (Utilities|Casting|CastToBP_MWBase (Variables|/Script/Engine.ChildActorComponent|GetChildActor (Variables|Default|GetBP_MWAgent2)))
        (:then
          (Variables|Default|SetAgent2 _asbp_mwbase_2)
          (Utilities|Array|Add (Variables|Default|GetAgents) 0)
          (Transformation|AttachComponentToComponent (Variables|/Script/Engine.Actor|GetRootComponent (Variables|Default|GetAgent1)) (Variables|Default|GetDefaultSceneRoot) "None" "KeepRelative" "KeepRelative" "KeepRelative" true)
          (Transformation|SetActorRelativeLocation (Variables|Default|GetAgent1) "150.000000,150.000000,88.000000")
          (Transformation|AttachComponentToComponent (Variables|/Script/Engine.Actor|GetRootComponent (Variables|Default|GetAgent2)) (Variables|Default|GetDefaultSceneRoot) "None" "KeepRelative" "KeepRelative" "KeepRelative" true)
          (Transformation|SetActorRelativeLocation (Variables|Default|GetAgent2) "150.000000,2250.000000,88.000000"))
        (:CastFailed
          (Development|PrintString "CastFailed" :!label _label))))
    (:CastFailed
      (goto _label))))

(event Collision|EventActorBeginOverlap
  (params (OtherActor :type Actor%20Object%20Reference)))

(event EventTick
  (params (DeltaSeconds :type Float%20%28single-precision%29)))

(fn ConstructionScript)