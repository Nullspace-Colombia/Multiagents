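; Base reinforcement-learning agent for a task where agents push a bar to a goal.
; Step counts frames and maps a discrete action to movement in four directions.
; State combines the capsule's XY position with hit normals from four world-axis line traces.
; Reward favors goal contact, then new closest bar-to-goal or agent-to-bar distances; episodes end on goal contact or frame limit, and reset repositions the bar.
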(event Custom|hitpush
  (params (Hit%20Component :type Primitive%20Component%20Object%20Reference) (Other%20Actor :type Actor%20Object%20Reference) (Other%20Component :type Primitive%20Component%20Object%20Reference) (Normal%20Impulse :type Vector) (Hit :type Hit%20Result%20Structure))
  (bind _returnvalue (Utilities|GetClass Other%20Actor))
  (if (== Other%20Actor (Variables|Default|Getgoal))
    (Variables|Default|SetDone (or (Variables|Default|GetDone) true))
    (Variables|Default|Settouch_goal true)
    (Development|PrintString "touched goal")
    (else
      (Variables|Default|SetDone (or (Variables|Default|GetDone) false))
      (if (or (== _returnvalue "/Game/Blueprints/WallMovement/BP_MWAgent1.BP_MWAgent1_C") (== _returnvalue "/Game/Blueprints/WallMovement/BP_MWAgent2.BP_MWAgent2_C"))
        (Variables|Default|Settouched true)
        (Development|PrintString "touched")
        (Development|PrintString (Utilities|GetDisplayName Other%20Actor))))))

(event Custom|print
  (Development|PrintString (Utilities|String|ToString(Vector) (Variables|/Script/Engine.SceneComponent|GetRelativeLocation (Variables|Collision|GetCapsuleComponent)))))

(event Custom|CustomEvent
  (params (ID :type Float%20%28double-precision%29))
  (Variables|Default|SetID ID))

(event EventMove
  (params (NewParam :type Float%20%28double-precision%29))
  (bind _returnvalue (Transformation|GetActorForwardVector))
  (bind _returnvalue_2 (Transformation|GetActorRightVector))
  ;[1 1 1] movement
  (if (== NewParam 0.0)
    (Pawn|Input|AddMovementInput _returnvalue_2 1.0 false)
    (elif (== NewParam 1.0)
      (Pawn|Input|AddMovementInput _returnvalue_2 -1.0 false)
      (elif (== NewParam 2.0)
        (Pawn|Input|AddMovementInput _returnvalue 1.0 false)
        (elif (== NewParam 3.0)
          (Pawn|Input|AddMovementInput _returnvalue -1.0 false))))))

(event Collision|EventActorBeginOverlap
  (params (OtherActor :type Actor%20Object%20Reference)))

(event EventStep
  (params (Action :type Float%20%28double-precision%29))
  ;[1 1 1] Step
  (Math|Integer|IncrementInt (Variables|Default|GetCounter)
    (:%20%20
      (CallFunction|Move Action))))

(event EventBeginPlay)

(fn ConstructionScript
  (bind _returnvalue (Rendering|Material|CreateDynamicMaterialInstance (Variables|Default|GetCube) 0 0 "None" :!class /Script/Engine.PrimitiveComponent))
  (Rendering|Material|SetVectorParameterValue _returnvalue "Param" (Variables|Default|GetColor) :!class /Script/Engine.MaterialInstanceDynamic))

(fn GetAgentState
  (bind _capsulecomponent (Variables|Collision|GetCapsuleComponent))
  (bind _relativelocation (Variables|/Script/Engine.SceneComponent|GetRelativeLocation _capsulecomponent))
  (bind _output_get (Variables|Default|Setobs (Utilities|Array|MakeArray (.x _relativelocation) (.y _relativelocation))))
  (bind _raytraces (|rayTracers)
    (:execute2
      (Utilities|Array|AppendArray _output_get _raytraces)
      (return (Variables|Default|Getobs)))))

(fn GetAgentReward
  (bind _goal (Variables|Default|Getgoal))
  (bind _capsulecomponent (Variables|Collision|GetCapsuleComponent))
  (bind _pushbar (Variables|Default|Getpushbar))
  (bind _relativelocation (Variables|/Script/Engine.SceneComponent|GetRelativeLocation _goal))
  (bind _relativelocation_2 (Variables|/Script/Engine.SceneComponent|GetRelativeLocation _capsulecomponent))
  (bind _relativelocation_3 (Variables|/Script/Engine.SceneComponent|GetRelativeLocation _pushbar))
  (bind _returnvalue (Math|Vector|Distance2D(Vector) (Math|Vector2D|MakeVector2D (.x _relativelocation) (.y _relativelocation)) (Math|Vector2D|MakeVector2D (.x _relativelocation_3) (.y _relativelocation_3))))
  (bind _returnvalue_2 (Math|Vector|Distance2D(Vector) (Math|Vector2D|MakeVector2D (.x _relativelocation_3) (.y _relativelocation_3)) (Math|Vector2D|MakeVector2D (.x _relativelocation_2) (.y _relativelocation_2))))
  (if (Variables|Default|Gettouch_goal)
    (Variables|Default|SetReward 5e+01)
    (Variables|Default|Settouch_goal false)
    (elif (Variables|Default|Gettouched)
      (Variables|Default|Settouched false)
      (if (<= _returnvalue (Variables|Default|Getprevious_distance_bar_goal))
        (Variables|Default|Setprevious_distance_bar_goal _returnvalue)
        (Variables|Default|SetReward 0.5)
        (else
          (Variables|Default|SetReward 0.0)))
      (elif (<= _returnvalue_2 (Variables|Default|Getprevious_distance_bar_agent))
        (Variables|Default|Setprevious_distance_bar_agent _returnvalue_2)
        (Variables|Default|SetReward 0.1)
        (else
          (Variables|Default|SetReward -0.1)))))
  (return (Variables|Default|GetReward)))

(fn IsAgentDone
  (Math|Integer|CompareInt (Variables|Default|GetCounter) (Variables|Default|GetMaxFrames)
    (:>
      (Variables|Default|SetDone (or (Variables|Default|GetDone) true) :!label _label)
      (Variables|Default|SetCounter 0))
    (:==
      (goto _label))
    (:<
      (Variables|Default|SetDone (or (Variables|Default|GetDone) false))))
  (return (Variables|Default|GetDone)))

(fn ResetAgent
  (Transformation|SetWorldLocationAndRotation (Variables|Default|Getpushbar) "0, 0, 0" "0, 0, 0" false false)
  (return 0))

(fn OnRepPushbar)

(fn GetID
  (return 0))

(fn GetReward
  (bind _agentreward (CallFunction|GetAgentReward))
  (return _agentreward))

(fn GetSelfActor
  (return self))

(fn GetState
  (bind _pos (CallFunction|GetAgentState))
  (return _pos))

(fn IsDone
  (bind _isagentdone (CallFunction|IsAgentDone))
  (return _isagentdone))

(fn Reset
  (bind _newactor (CallFunction|ResetAgent))
  (Variables|Default|SetDone false)
  (return _newactor false))