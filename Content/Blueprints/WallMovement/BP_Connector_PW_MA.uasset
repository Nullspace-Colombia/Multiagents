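; BP_Connector_PW_MA bridges multiple BI_Agent actors to an external reinforcement-learning client through a local server.
; BeginPlay collects agents, starts the server and sets time dilation, with Enhanced Input for manually moving two agents.
; Received actions open a gate that Tick passes through to step agents or reset finished ones, replacing actors when needed.
; Each step sends observations, rewards and done flags, then closes the gate until new data arrives.
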(event Custom|SetAgents
  ;[1 1 1] SetAgents
  (for _array_element (Variables|Default|GetActorAgents)
    (bind _asbi_agent (Utilities|Casting|CastToBI_Agent _array_element))
    (Utilities|Array|Add (Variables|Default|GetAgents) _asbi_agent)))

(event Custom|SendAgents
  ;[1 1 1] Send Angents Info
  (Class|Pole|SendMultiagentsInfo (Variables|Default|GetAgentsInfo))
  (Utilities|Array|Clear (Variables|Default|GetAgentsInfo)))

(event Custom|StartConnection
  ;[0.4158 0.6112 1] Start Connection
  (|SyncData)
  (Class|Pole|StartServer "127.0.0.1" 10010))

(event Custom|Step
  ;[1 1 1] step
  (for (_array_element _array_index) (Variables|Default|GetAgents)
    (if (Utilities|Array|Get(acopy) (Variables|Default|GetIsDone_Agents) _array_index)
      (bind (_newactor _bcreateactor) (Default|Reset _array_element))
      (if _bcreateactor
        (bind _actor (Default|GetSelfActor _array_element))
        (Actor|DestroyActor _actor)
        (Utilities|Array|SetArrayElem (Variables|Default|GetAgents) _array_index _newactor)
        (bind _observations (Default|GetState _array_element :!label _label))
        (bind _bdone (Default|IsDone _array_element))
        (bind _reward (Default|GetReward _array_element))
        (bind _returnvalue (Class|Pole|AddAgent _array_index _observations _reward _bdone))
        (Utilities|Array|AppendArray (Variables|Default|GetAgentsInfo) _returnvalue)
        (Utilities|Array|SetArrayElem (Variables|Default|GetIsDone_Agents) _array_index _bdone))
      (else
        (Default|Step _array_element (Utilities|Array|Get(acopy) (Variables|Default|GetActions) _array_index))
        (goto _label))))
  (CallFunction|SendAgents)
  (CallFunction|CloseGate))

(event Input|EnhancedActionEvents|EnhancedInputActionIA_MoveLeft
  (params (ActionValue :type Boolean) (ElapsedSeconds :type Float%20%28double-precision%29) (TriggeredSeconds :type Float%20%28double-precision%29) (InputAction :type Input%20Action%20Object%20Reference :default "/Game/Inputs/IA_MoveLeft.IA_MoveLeft"))
  ;[1 1 1] inputs
  (:Triggered
    (Default|Move (Utilities|Array|Get(acopy) (Variables|Default|GetAgents)) 1.0)))

(event Input|EnhancedActionEvents|EnhancedInputActionIA_MoveRight
  (params (ActionValue :type Boolean) (ElapsedSeconds :type Float%20%28double-precision%29) (TriggeredSeconds :type Float%20%28double-precision%29) (InputAction :type Input%20Action%20Object%20Reference :default "/Game/Inputs/IA_MoveRight.IA_MoveRight"))
  ;[1 1 1] inputs
  (:Triggered
    (Default|Move (Utilities|Array|Get(acopy) (Variables|Default|GetAgents)) 0.0)))

(event Input|EnhancedActionEvents|EnhancedInputActionIA_MoveUp_2
  (params (ActionValue :type Boolean) (ElapsedSeconds :type Float%20%28double-precision%29) (TriggeredSeconds :type Float%20%28double-precision%29) (InputAction :type Input%20Action%20Object%20Reference :default "/Game/Inputs/IA_MoveUp_2.IA_MoveUp_2"))
  ;[1 1 1] inputs
  (:Triggered
    (Default|Move (Utilities|Array|Get(acopy) (Variables|Default|GetAgents) 1) 2.0)))

(event Input|EnhancedActionEvents|EnhancedInputActionIA_MoveDown_2
  (params (ActionValue :type Boolean) (ElapsedSeconds :type Float%20%28double-precision%29) (TriggeredSeconds :type Float%20%28double-precision%29) (InputAction :type Input%20Action%20Object%20Reference :default "/Game/Inputs/IA_MoveDown_2.IA_MoveDown_2"))
  ;[1 1 1] inputs
  (:Triggered
    (Default|Move (Utilities|Array|Get(acopy) (Variables|Default|GetAgents) 1) 3.0)))

(event Input|EnhancedActionEvents|EnhancedInputActionIA_MoveDown
  (params (ActionValue :type Boolean) (ElapsedSeconds :type Float%20%28double-precision%29) (TriggeredSeconds :type Float%20%28double-precision%29) (InputAction :type Input%20Action%20Object%20Reference :default "/Game/Inputs/IA_MoveDown.IA_MoveDown"))
  ;[1 1 1] inputs
  (:Triggered
    (Default|Move (Utilities|Array|Get(acopy) (Variables|Default|GetAgents)) 3.0)))

(event Input|EnhancedActionEvents|EnhancedInputActionIA_MoveUp
  (params (ActionValue :type Boolean) (ElapsedSeconds :type Float%20%28double-precision%29) (TriggeredSeconds :type Float%20%28double-precision%29) (InputAction :type Input%20Action%20Object%20Reference :default "/Game/Inputs/IA_MoveUp.IA_MoveUp"))
  ;[1 1 1] inputs
  (:Triggered
    (Default|Move (Utilities|Array|Get(acopy) (Variables|Default|GetAgents)) 2.0)))

(event Input|EnhancedActionEvents|EnhancedInputActionIA_MoveRight_2
  (params (ActionValue :type Boolean) (ElapsedSeconds :type Float%20%28double-precision%29) (TriggeredSeconds :type Float%20%28double-precision%29) (InputAction :type Input%20Action%20Object%20Reference :default "/Game/Inputs/IA_MoveRight_2.IA_MoveRight_2"))
  ;[1 1 1] inputs
  (:Triggered
    (Default|Move (Utilities|Array|Get(acopy) (Variables|Default|GetAgents) 1) 0.0)))

(event Input|EnhancedActionEvents|EnhancedInputActionIA_MoveLeft_2
  (params (ActionValue :type Boolean) (ElapsedSeconds :type Float%20%28double-precision%29) (TriggeredSeconds :type Float%20%28double-precision%29) (InputAction :type Input%20Action%20Object%20Reference :default "/Game/Inputs/IA_MoveLeft_2.IA_MoveLeft_2"))
  ;[1 1 1] inputs
  (:Triggered
    (Default|Move (Utilities|Array|Get(acopy) (Variables|Default|GetAgents) 1) 1.0)))

(event EventTick
  (params (DeltaSeconds :type Float%20%28single-precision%29))
  (CallFunction|Hop))

(event EventBeginPlay
  (CallFunction|SetAgents)
  (CallFunction|StartConnection)
  (Utilities|Time|SetGlobalTimeDilation (Variables|Default|GetTime%20Dilation))
  (bind _asplayer_controller (Utilities|Casting|CastToPlayerController (Pawn|GetController)))
  (Utilities|IsValid (PlayerController|LocalPlayerSubsystems|GetEnhancedInputLocalPlayerSubsystem _asplayer_controller)
    (:Is%20Valid
      (Input|AddMappingContext (PlayerController|LocalPlayerSubsystems|GetEnhancedInputLocalPlayerSubsystem _asplayer_controller) "/Game/Inputs/IMC_Arena.IMC_Arena" 0 "(bIgnoreAllPressedKeysUntilRelease=True,bForceImmediately=False)"))))

(fn ConstructionScript)

(event Custom|Open_Gate
  (Utilities|FlowControl|Gate true) ; enters at Open
)

(event Custom|Close_Gate
  (Utilities|FlowControl|Gate true) ; enters at Close
)

(event Custom|Hop
  (Class|Pole|ConductConnection)
  (if (Variables|Default|Getconnected)
    (Utilities|FlowControl|Gate true
      (:Exit
        (CallFunction|Step)))))

(event Custom|OnDataReceptionDelegate_Event_0
  (params (Arr :type Array%20of%20Bytes))
  (bind _returnvalue (Class|Pole|GetAction Arr))
  (Variables|Default|SetActions _returnvalue)
  (CallFunction|OpenGate))