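; BP_MWAgent2 is the second agent in the WallMovement task, a child Blueprint that appears to serve a reinforcement-learning style step, reward and reset loop.
; Stepping, movement, state, reward and done checks defer to the parent class.
; Reset respawns it at a random spot within the scenario's X range and its own Y band, zeroes velocity and episode variables, then records starting agent-bar and bar-goal distances.
; Outlimited respawns it when flagged out of bounds.
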(event EventSetID
  (params (ID :type Integer))
  (|CallParentFunction ID))

(event EventBeginPlay
  (|CallParentFunction))

(event EventStep
  (params (Action :type Array%20of%20Floats%20%28double-precision%29))
  ;[1 1 1] Step
  (|CallParentFunction Action))

(event EventSetActionID
  (params (ActionID :type Integer))
  (|CallParentFunction ActionID))

(event Collision|EventActorBeginOverlap
  (params (OtherActor :type Actor%20Object%20Reference))
  (|CallParentFunction OtherActor) ; This node is disabled and will not be called.\nDrag off pins to build functionality.
)

(event EventMove
  (params (NewParam :type Float%20%28double-precision%29))
  (|CallParentFunction NewParam))

(fn ConstructionScript
  (|CallParentFunction))

(fn GetAgentReward
  (bind _agentreward (|CallParentFunction))
  (return _agentreward))

(fn ResetAgent
  (bind _agent (CallFunction|GetEscenario))
  (Transformation|SetActorRelativeLocation (Math|Vector|MakeVector (Math|Random|RandomFloatinRange (Utilities|Array|Get(acopy) _agent) (Utilities|Array|Get(acopy) _agent 1)) (Math|Random|RandomFloatinRange 1.5e+03 2.25e+03) 1e+02))
  (Transformation|SetActorRelativeRotation "0, 0, 0")
  (Class|PrimitiveComponent|SetAllPhysicsLinearVelocity (Variables|Default|GetCapsuleComponent) "0, 0, 0" false)
  (return self))

(fn GetState
  (bind _pos (CallFunction|GetAgentState))
  (return _pos))

(fn GetAgentState
  (bind _pos (|CallParentFunction))
  (return _pos))

(fn IsDone
  (bind _isagentdone (CallFunction|IsAgentDone))
  (return _isagentdone))

(fn GetSelfActor
  (return self))

(fn Reset
  (bind _newactor (CallFunction|ResetAgent))
  (Variables|Default|SetDone false)
  (Variables|Default|SetReward 0.0)
  (Variables|Default|SetCounter 0)
  (bind (_bar_agent _bar_goal) (CallFunction|Distances))
  (bind _output_get (Variables|Default|Setfirst_bar_goal _bar_goal))
  (bind _output_get_2 (Variables|Default|Setfirst_agent_bar _bar_agent))
  (Development|PrintString (Utilities|String|Append "first agent bar agent 2:" (Utilities|String|ToString(Float) _output_get_2) "first bar goal agent 2: " (Utilities|String|ToString(Float) _output_get)) false false "(R=0.000000,G=0.660000,B=1.000000,A=1.000000)" 2e+01)
  (return _newactor false))

(fn GetReward
  (bind _agentreward (CallFunction|GetAgentReward))
  (return _agentreward))

(fn IsAgentDone
  (bind _isagentdone (|CallParentFunction))
  (return _isagentdone))

(fn Outlimited
  (if (Variables|Default|Getout_limits)
    (CallFunction|ResetAgent)
    (Variables|Default|Setout_limits false)
    (Development|PrintString "was outlimits" true false "(R=0.000000,G=0.660000,B=1.000000,A=1.000000)" 2e+01)))