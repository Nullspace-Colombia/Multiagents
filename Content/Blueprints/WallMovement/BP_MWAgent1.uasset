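; BP_MWAgent1 is a reinforcement-learning agent (ID 0) in the WallMovement environment, built on a parent agent with a pushbar and goal.
; Step, movement, reward and done checks defer to the parent, while the state appends bar and goal X/Y positions to the parent's observations.
; Reset randomizes agent, bar and goal placement from scenario ranges, varies bar and goal scale, clears bar velocity and records initial agent-bar and bar-goal distances.
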(event Custom|SetID_1
  (params (ID :type Float%20%28double-precision%29)))

(event EventSetID
  (params (ID :type Integer))
  (|CallParentFunction ID))

(event EventMove
  (params (NewParam :type Float%20%28double-precision%29))
  (|CallParentFunction NewParam))

(event EventBeginPlay
  (|CallParentFunction))

(event EventStep
  (params (Action :type Array%20of%20Floats%20%28double-precision%29))
  ;[1 1 1] Step
  (|CallParentFunction Action))

(event EventSetActionID
  (params (ActionID :type Integer))
  (|CallParentFunction ActionID))

(event Collision|EventActorBeginOverlap
  (params (OtherActor :type Actor%20Object%20Reference))
  (|CallParentFunction OtherActor) ; This node is disabled and will not be called.\nDrag off pins to build functionality.
)

(fn ConstructionScript
  (|CallParentFunction))

(fn GetAgentReward
  (bind _agentreward (|CallParentFunction))
  (return _agentreward))

(fn ResetAgent
  (bind _agent (CallFunction|GetEscenario))
  (Transformation|SetActorRelativeLocation (Math|Vector|MakeVector (Math|Random|RandomFloatinRange (Utilities|Array|Get(acopy) _agent) (Utilities|Array|Get(acopy) _agent 1)) (Math|Random|RandomFloatinRange 2.5e+02 1.2e+03) 1e+02))
  (Transformation|SetActorRelativeRotation "0, 0, 0")
  (return self))

(fn GetState
  (bind _pos (CallFunction|GetAgentState))
  (return _pos))

(fn GetAgentState
  (bind _pushbar (Variables|Default|Getpushbar))
  (bind _goal (Variables|Default|Getgoal))
  (bind (_barposition_x _barposition_y _barscale_x _barscale_y _goalposition_x _goalposition_y) (|Positions _pushbar _goal))
  (bind _pos (|CallParentFunction))
  (bind _output_get (Variables|Default|Setobs_0 _pos))
  (Utilities|Array|AppendArray _output_get (Utilities|Array|MakeArray _barposition_x _barposition_y _goalposition_x _goalposition_y))
  (return (Variables|Default|Getobs_0)))

(fn IsDone
  (bind _isagentdone (CallFunction|IsAgentDone))
  (return _isagentdone))

(fn GetSelfActor
  (return self))

(fn Reset
  (bind _pushbar (Variables|Default|Getpushbar))
  (bind _newactor (CallFunction|ResetAgent))
  (bind _bar (CallFunction|GetEscenario))
  (Variables|Default|SetDone false)
  (Transformation|SetRelativeTransform _pushbar (Math|Transform|MakeTransform (Math|Vector|MakeVector (Math|Random|RandomFloatinRange (Utilities|Array|Get(acopy) _bar) (Utilities|Array|Get(acopy) _bar 1)) (Math|Random|RandomFloatinRange 4.5e+02 1.65e+03) 9e+01) (Math|Rotator|MakeRotator 0.0 0.0 (Math|Random|RandomFloatinRange 0.0 25.0)) (Math|Vector|MakeVector (Math|Random|RandomFloatinRange 0.2 0.3) (Math|Random|RandomFloatinRange 5.0 8.0) 2.0)) false false)
  (Class|PrimitiveComponent|SetPhysicsAngularVelocityinDegrees _pushbar "0, 0, 0" false "None")
  (Physics|SetPhysicsLinearVelocity _pushbar "0, 0, 0" false "None")
  (bind _goal (CallFunction|GetEscenario))
  (Transformation|SetRelativeTransform (Variables|Default|Getgoal) (Math|Transform|MakeTransform (Math|Vector|MakeVector (Math|Random|RandomFloatinRange (Utilities|Array|Get(acopy) _goal) (Utilities|Array|Get(acopy) _goal 1)) (Math|Random|RandomFloatinRange 4.5e+02 1.95e+03) -5.0) "90.000000,180.000000,180.000000" (Math|Vector|MakeVector (Math|Random|RandomFloatinRange 0.09 0.2) (Math|Random|RandomFloatinRange 5.0 8.0) 1.0)) false false)
  (Variables|Default|SetReward 0.0)
  (Variables|Default|SetCounter 0)
  (bind (_bar_agent _bar_goal) (CallFunction|Distances))
  (bind _output_get (Variables|Default|Setfirst_bar_goal _bar_goal))
  (bind _output_get_2 (Variables|Default|Setfirst_agent_bar _bar_agent))
  (Development|PrintString (Utilities|String|Append "first agent bar agent 1:" (Utilities|String|ToString(Float) _output_get_2) "first bar goal agent 1" (Utilities|String|ToString(Float) _output_get)) false false "(R=0.000000,G=0.660000,B=1.000000,A=1.000000)" 2e+01)
  (return _newactor false))

(fn GetReward
  (bind _agentreward (CallFunction|GetAgentReward))
  (return _agentreward))

(fn IsAgentDone
  (bind _isagentdone (|CallParentFunction))
  (return _isagentdone))

(fn GetID
  (return 0))

(fn Outlimited
  (if (Variables|Default|Getout_limits)
    (CallFunction|ResetAgent)
    (Variables|Default|Setout_limits false)
    (Development|PrintString "was outlimits" true false "(R=0.000000,G=0.660000,B=1.000000,A=1.000000)" 2e+01)))