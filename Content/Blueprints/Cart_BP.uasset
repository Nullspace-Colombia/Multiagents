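; Cart Blueprint that hosts a local socket server to receive external data and print it on screen for debugging.
; BeginPlay binds the data-reception delegate and starts the server, Tick services the connection, and each received array is parsed and printed element by element.
; The Right key sets movement and direction variables that nothing live reads; the data-driven sideways offset logic is disconnected and never runs.
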(event Custom|OnDataReceptionDelegate_Event_0
  (params (Arr :type Array%20of%20Bytes))
  (bind _returnvalue (Class|Pole|ParseData Arr))
  (for (_array_element _array_index) _returnvalue
    (Development|PrintString (Utilities|String|Append "[" (Utilities|String|ToString(Integer) _array_index) "];" (Utilities|String|ToString(Float) _array_element)) true false "(R=1.000000,G=0.055645,B=0.305520,A=1.000000)" 2e+01)))

(event EventBeginPlay
  (EventDispatchers|AssignOnDataReceptionDelegate (delegate Custom|OnDataReceptionDelegate_Event_0))
  (Class|Pole|StartServer "127.0.0.1" 10000))

(event Collision|EventActorBeginOverlap
  (params (OtherActor :type Actor%20Object%20Reference)))

(event EventTick
  (params (DeltaSeconds :type Float%20%28single-precision%29))
  (Class|Pole|ConductConnection))

(event Input|KeyboardEvents|Right
  (params (Key :type Key%20Structure :default "None"))
  (:Pressed
    (Variables|Default|SetisMoving true)
    (Variables|Default|SetisLeft false)
    (Variables|Default|SetdirText "Right"))
  (:Released
    (Variables|Default|SetisMoving false)))

(fn ConstructionScript)