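; BI_Agent is a Blueprint interface for agents in a reinforcement-learning style loop.
; It declares Step with an action, state and reward queries, a done check, and a Reset that reports whether to create a new actor.
; It also exposes the owning actor, an agent ID getter and setter, and an action ID setter, leaving all logic to implementers.
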(fn Step
  (params (Action :type Array%20of%20Floats%20%28double-precision%29)))

(fn GetState
  (return 0))

(fn Reset
  (return 0 false))

(fn IsDone
  (return false))

(fn GetReward
  (return 0.0))

(fn GetSelfActor
  (return 0))

(fn GetID
  (return 0))

(fn SetID
  (params (ID :type Integer)))

(fn SetActionID
  (params (ActionID :type Integer)))