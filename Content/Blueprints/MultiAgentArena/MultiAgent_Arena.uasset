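; MultiAgent_Arena is an arena actor that sets up two BP_ArenaAgentBase agents from child actor components.
; On BeginPlay it casts and stores both agents, attaches them to its root and places them at opposite corners of a 700-unit square.
; It passes each agent movement limits derived from its position, with both using Agent1's location as the shared offset.
; A failed cast only prints an error.
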(event EventBeginPlay
  (bind _asbp_arena_agent_base (Utilities|Casting|CastToBP_ArenaAgentBase (Variables|/Script/Engine.ChildActorComponent|GetChildActor (Variables|Default|GetBP_ArenaAgent1)))
    (:then
      (Variables|Default|SetAgent1 _asbp_arena_agent_base)
      (Utilities|Array|Add (Variables|Default|GetAgents) _asbp_arena_agent_base)
      (bind _asbp_arena_agent_base_2 (Utilities|Casting|CastToBP_ArenaAgentBase (Variables|/Script/Engine.ChildActorComponent|GetChildActor (Variables|Default|GetBP_ArenaAgent2)))
        (:then
          (Variables|Default|SetAgent2 _asbp_arena_agent_base_2)
          (Utilities|Array|Add (Variables|Default|GetAgents) _asbp_arena_agent_base_2)
          (Transformation|AttachComponentToComponent (Variables|/Script/Engine.Actor|GetRootComponent (Variables|Default|GetAgent1)) (Variables|Default|GetDefaultSceneRoot) "None" "KeepRelative" "KeepRelative" "KeepRelative" true)
          (Transformation|SetActorRelativeLocation (Variables|Default|GetAgent1))
          (Transformation|AttachComponentToComponent (Variables|/Script/Engine.Actor|GetRootComponent (Variables|Default|GetAgent2)) (Variables|Default|GetDefaultSceneRoot) "None" "KeepRelative" "KeepRelative" "KeepRelative" true)
          (Transformation|SetActorRelativeLocation (Variables|Default|GetAgent2) "700.000000,700.000000,0.000000")
          (Default|SetLimits (Variables|Default|GetAgent1) (+ (.x (.location (Transformation|GetActorTransform (Variables|Default|GetAgent1)))) 7e+02) (.x (.location (Transformation|GetActorTransform (Variables|Default|GetAgent1)))) (+ (.y (.location (Transformation|GetActorTransform (Variables|Default|GetAgent1)))) 7e+02) (.y (.location (Transformation|GetActorTransform (Variables|Default|GetAgent1)))) (.x (.location (Transformation|GetActorTransform (Variables|Default|GetAgent1)))) (.y (.location (Transformation|GetActorTransform (Variables|Default|GetAgent1)))))
          (Default|SetLimits (Variables|Default|GetAgent2) (.x (.location (Transformation|GetActorTransform (Variables|Default|GetAgent2)))) (+ (.x (.location (Transformation|GetActorTransform (Variables|Default|GetAgent2)))) -7e+02) (.y (.location (Transformation|GetActorTransform (Variables|Default|GetAgent2)))) (+ (.y (.location (Transformation|GetActorTransform (Variables|Default|GetAgent2)))) -7e+02) (.x (.location (Transformation|GetActorTransform (Variables|Default|GetAgent1)))) (.y (.location (Transformation|GetActorTransform (Variables|Default|GetAgent1))))))
        (:CastFailed
          (Development|PrintString "CastFailed" :!label _label))))
    (:CastFailed
      (goto _label))))

(event Collision|EventActorBeginOverlap
  (params (OtherActor :type Actor%20Object%20Reference))
  (|CallParentFunction OtherActor) ; This node is disabled and will not be called.\nDrag off pins to build functionality.
)

(event EventTick
  (params (DeltaSeconds :type Float%20%28single-precision%29))
  (|CallParentFunction DeltaSeconds) ; This node is disabled and will not be called.\nDrag off pins to build functionality.
)

(fn ConstructionScript)