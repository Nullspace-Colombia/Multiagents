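; Grid-stepping arena agent that appears built for reinforcement learning, driven by Step actions or Enhanced Input keys.
; Both inputs feed AddLateralMovement, which teleports one cell within X/Y limits.
; GetState encodes position as an eight-wide cell index, adding it to Visited before the known-field check, so it always reads known.
; Reward derives from collision and that flag, IsDone caps step count, and Reset spawns a fresh agent.
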(event Custom|AddLateralMovement
  (params (Input :type Float%20%28double-precision%29))
  ;[0.5697 1 0.4631] Actions
  (CallFunction|CheckLimitsX)
  (CallFunction|CheckLimitsY)
  (if (and (== Input 0.0) (not (Variables|Default|GetIsOverLimitUp)))
    (Transformation|SetActorLocation (+ (Transformation|GetActorLocation) (Math|Vector|MakeVector 0.0 -1e+02 0.0)) false false)
    (elif (and (== Input 2.0) (not (Variables|Default|GetIsOverLimitDown)))
      (Transformation|SetActorLocation (+ (Transformation|GetActorLocation) (Math|Vector|MakeVector 0.0 1e+02 0.0)) false false)
      (elif (and (== Input 1.0) (not (Variables|Default|GetIsOverLimitRight)))
        (Transformation|SetActorLocation (+ (Transformation|GetActorLocation) (Math|Vector|MakeVector 1e+02 0.0 0.0)) false false)
        (elif (and (== Input 3.0) (not (Variables|Default|GetIsOverLimitLeft)))
          (Transformation|SetActorLocation (+ (Transformation|GetActorLocation) (Math|Vector|MakeVector -1e+02 0.0 0.0)) false false)
          (else
            (Transformation|SetActorLocation (Transformation|GetActorLocation) false false)))))))

(event Custom|CheckLimitsY
  (bind _returnvalue (Transformation|GetActorLocation))
  ;[1 1 1] Check Limits
  (Math|Float|CompareFloat (+ (.y _returnvalue) 1e+02) (Variables|Default|GetYLimH)
    (:>
      (Variables|Default|SetIsOverLimitDown true))
    (:==
      (Variables|Default|SetIsOverLimitDown false :!label _label))
    (:<
      (goto _label)))
  (Math|Float|CompareFloat (+ (.y _returnvalue) -1e+02) (Variables|Default|GetYLimL)
    (:>
      (Variables|Default|SetIsOverLimitUp false :!label _label_2))
    (:==
      (goto _label_2))
    (:<
      (Variables|Default|SetIsOverLimitUp true))))

(event Custom|CheckLimitsX
  (bind _returnvalue (Transformation|GetActorLocation))
  ;[1 1 1] Check Limits
  (Math|Float|CompareFloat (+ (.x _returnvalue) 1e+02) (Variables|Default|GetXLimH)
    (:>
      (Variables|Default|SetIsOverLimitRight true))
    (:==
      (Variables|Default|SetIsOverLimitRight false :!label _label))
    (:<
      (goto _label)))
  (Math|Float|CompareFloat (+ (.x _returnvalue) -1e+02) (Variables|Default|GetXLimL)
    (:>
      (Variables|Default|SetIsOverLimitLeft false :!label _label_2))
    (:==
      (goto _label_2))
    (:<
      (Variables|Default|SetIsOverLimitLeft true))))

(event Input|EnhancedActionEvents|EnhancedInputActionIA_MoveLeft
  (params (ActionValue :type Boolean) (ElapsedSeconds :type Float%20%28double-precision%29) (TriggeredSeconds :type Float%20%28double-precision%29) (InputAction :type Input%20Action%20Object%20Reference :default "/Game/Inputs/IA_MoveLeft.IA_MoveLeft"))
  ;[0.5697 1 0.4631] Actions
  (:Triggered
    (CallFunction|AddLateralMovement 3.0)))

(event Input|EnhancedActionEvents|EnhancedInputActionIA_MoveRight
  (params (ActionValue :type Boolean) (ElapsedSeconds :type Float%20%28double-precision%29) (TriggeredSeconds :type Float%20%28double-precision%29) (InputAction :type Input%20Action%20Object%20Reference :default "/Game/Inputs/IA_MoveRight.IA_MoveRight"))
  ;[0.5697 1 0.4631] Actions
  (:Triggered
    (CallFunction|AddLateralMovement 1.0)))

(event Input|EnhancedActionEvents|EnhancedInputActionIA_MoveDown
  (params (ActionValue :type Boolean) (ElapsedSeconds :type Float%20%28double-precision%29) (TriggeredSeconds :type Float%20%28double-precision%29) (InputAction :type Input%20Action%20Object%20Reference :default "/Game/Inputs/IA_MoveDown.IA_MoveDown"))
  ;[0.5697 1 0.4631] Actions
  (:Triggered
    (CallFunction|AddLateralMovement 2.0)))

(event Input|EnhancedActionEvents|EnhancedInputActionIA_MoveUp
  (params (ActionValue :type Boolean) (ElapsedSeconds :type Float%20%28double-precision%29) (TriggeredSeconds :type Float%20%28double-precision%29) (InputAction :type Input%20Action%20Object%20Reference :default "/Game/Inputs/IA_MoveUp.IA_MoveUp"))
  ;[0.5697 1 0.4631] Actions
  (:Triggered
    (CallFunction|AddLateralMovement 0.0)))

(event EventBeginPlay
  ;[1 1 1] Configure
  (bind _asplayer_controller (Utilities|Casting|CastToPlayerController (Pawn|GetController)))
  (Utilities|IsValid (PlayerController|LocalPlayerSubsystems|GetEnhancedInputLocalPlayerSubsystem _asplayer_controller)
    (:Is%20Valid
      (Input|AddMappingContext (PlayerController|LocalPlayerSubsystems|GetEnhancedInputLocalPlayerSubsystem _asplayer_controller) "/Game/Inputs/IMC_Arena.IMC_Arena" 0 "(bIgnoreAllPressedKeysUntilRelease=True,bForceImmediately=False)")
      (Pawn|Components|CharacterMovement|SetMovementMode (Variables|Character|GetCharacterMovement) "MOVE_Flying" 0))))

(event EventTick
  (params (DeltaSeconds :type Float%20%28single-precision%29)))

(event EventStep
  (params (Action :type Array%20of%20Floats%20%28double-precision%29))
  ;[1 1 1] Step
  (Math|Integer|IncrementInt (Variables|Default|GetCounter)
    (:%20%20
      (CallFunction|AddLateralMovement (Utilities|Array|Get(acopy) Action)))))

(event Collision|EventActorBeginOverlap
  (params (OtherActor :type Actor%20Object%20Reference))
  ;[1 1 1] Check Collision
  (Variables|Default|Setcollision true))

(fn ConstructionScript
  (bind _returnvalue (Rendering|Material|CreateDynamicMaterialInstance (Variables|Default|GetCube) 0 0 "None" :!class /Script/Engine.PrimitiveComponent))
  (Rendering|Material|SetVectorParameterValue _returnvalue "Param" (Variables|Default|GetColor) :!class /Script/Engine.MaterialInstanceDynamic))

(fn GetAgentState
  (params (Agent :type Actor%20Object%20Reference))
  (bind _returnvalue (Transformation|GetActorLocation Agent))
  (return (+ (Math|Float|SafeDivide (Math|Float|Absolute(Float) (- (.x _returnvalue) 1.85e+03)) 1e+02) (* (Math|Float|SafeDivide (Math|Float|Absolute(Float) (- (.y _returnvalue) 3.5e+02)) 1e+02) 8.0))))

(fn GetAgentReward
  (if (Variables|Default|Getcollision)
    (Variables|Default|SetReward -1.0)
    (return (Variables|Default|GetReward))
    (elif (Variables|Default|GetisKnownField)
      (Variables|Default|SetReward -0.5)
      (else
        (Variables|Default|SetReward 1.0)))))

(fn GetID
  (return 0.0))

(fn GetReward
  (bind _agentreward (CallFunction|GetAgentReward))
  (return _agentreward))

(fn GetSelfActor
  (return self))

(fn GetState
  (bind _returnvalue (Transformation|GetActorLocation))
  (bind _returnvalue_2 (Math|Float|Absolute(Float) (.x _returnvalue)))
  (bind _returnvalue_3 (Math|Float|Absolute(Float) (.y _returnvalue)))
  (bind _returnvalue_4 (- _returnvalue_2 5e+01))
  (bind _returnvalue_5 (- _returnvalue_3 5e+01))
  (bind _returnvalue_6 (Math|Float|SafeDivide _returnvalue_4 1e+02))
  (bind _returnvalue_7 (Math|Float|SafeDivide _returnvalue_5 1e+02))
  (bind _returnvalue_8 (* _returnvalue_7 8.0))
  (bind _returnvalue_9 (+ _returnvalue_6 _returnvalue_8))
  (Utilities|Array|Add (Variables|Default|GetVisited) _returnvalue_9)
  (Variables|Default|SetisKnownField (Utilities|Array|ContainsItem (Variables|Default|GetVisited) _returnvalue_9))
  (return (Utilities|Array|MakeArray _returnvalue_9)))

(fn IsDone
  (Math|Integer|CompareInt (Variables|Default|GetCounter) (Variables|Default|GetMaxFrames)
    (:>
      (Variables|Default|SetDone true :!label _label)
      (Variables|Default|SetCounter 0))
    (:==
      (goto _label))
    (:<
      (Variables|Default|SetDone false)))
  (return (Variables|Default|GetDone)))

(fn Reset
  (bind _returnvalue (Game|SpawnActorfromClass "BP_ArenaAgent_C" (Math|Transform|MakeTransform (Math|Vector|MakeVector 5e+01 5e+01 (.z (Transformation|GetActorLocation))) "0, 0, 0" "1.000000,1.000000,1.000000") "AlwaysSpawn" 0 0))
  (return _returnvalue true))