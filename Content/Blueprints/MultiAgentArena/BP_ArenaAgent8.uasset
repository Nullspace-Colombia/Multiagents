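; BP_ArenaAgent8 is a child agent Blueprint for a multi-agent arena with a step, state, reward, done and reset interface, apparently for reinforcement learning.
; Stepping, movement, state and done checks defer to the parent.
; A Hit event sets a collision flag that turns a small per-step penalty into a positive reward; nothing here clears it.
; Reset teleports this same actor to its own hardcoded start location.
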(event EventBeginPlay
  (|CallParentFunction) ; This node is disabled and will not be called.\nDrag off pins to build functionality.
)

(event Collision|EventHit
  (params (MyComp :type Primitive%20Component%20Object%20Reference) (Other :type Actor%20Object%20Reference) (OtherComp :type Primitive%20Component%20Object%20Reference) (bSelfMoved :type Boolean) (HitLocation :type Vector :default "0, 0, 0") (HitNormal :type Vector :default "0, 0, 0") (NormalImpulse :type Vector :default "0, 0, 0") (Hit :type Hit%20Result%20Structure%20%28by%20ref%29))
  ;[1 1 1] Check Collision
  (Variables|Default|Setcollision true))

(event EventTick
  (params (DeltaSeconds :type Float%20%28single-precision%29))
  (|CallParentFunction DeltaSeconds) ; This node is disabled and will not be called.\nDrag off pins to build functionality.
)

(event EventSetScenario
  (params (scenario :type Integer)))

(event EventStep
  (params (Action :type Array%20of%20Floats%20%28double-precision%29))
  (|CallParentFunction Action))

(event EventMove
  (params (NewParam :type Float%20%28double-precision%29))
  (|CallParentFunction NewParam))

(event Collision|EventActorBeginOverlap
  (params (OtherActor :type Actor%20Object%20Reference))
  (|CallParentFunction OtherActor) ; This node is disabled and will not be called.\nDrag off pins to build functionality.
)

(event EventSetID
  (params (ID :type Integer))
  (|CallParentFunction ID))

(event EventSetActionID
  (params (ActionID :type Integer))
  (|CallParentFunction ActionID))

(fn ConstructionScript
  (|CallParentFunction))

(fn GetAgentReward
  (if (Variables|Default|Getcollision)
    (Variables|Default|SetReward 1.0)
    (else
      (Variables|Default|SetReward -0.1)))
  (return (Variables|Default|GetReward)))

(fn ResetAgent
  (Transformation|SetActorLocation (Math|Vector|MakeVector 1e+03 2e+03 0.0) false true)
  (return self))

(fn GetState
  (bind _observations (|CallParentFunction))
  (return _observations))

(fn GetAgentState
  (bind _pos (|CallParentFunction))
  (return _pos))

(fn IsDone
  (bind _isagentdone (CallFunction|IsAgentDone))
  (return _isagentdone))

(fn GetSelfActor
  (return self))

(fn Reset
  (bind _newactor (CallFunction|ResetAgent))
  (return _newactor true))

(fn GetReward
  (bind _agentreward (CallFunction|GetAgentReward))
  (return _agentreward))

(fn IsAgentDone
  (bind _isagentdone (|CallParentFunction))
  (return _isagentdone))

(fn GetID
  (return (Variables|Default|GetID)))