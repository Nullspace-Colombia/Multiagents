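; BP_ArenaAgent3 is a multi-agent arena agent, apparently for reinforcement learning, that moves laterally using the third action element on each Step.
; Its state is an 8-wide grid cell index from location, added to Visited before the known-field check, so that check always passes.
; Reward penalizes collisions most, then known fields, and otherwise is positive.
; Reset spawns a BP_ArenaAgent1, rather than its own class, and done checks defer to the parent.
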(event EventBeginPlay
  (|CallParentFunction) ; This node is disabled and will not be called.\nDrag off pins to build functionality.
)

(event Collision|EventHit
  (params (MyComp :type Primitive%20Component%20Object%20Reference) (Other :type Actor%20Object%20Reference) (OtherComp :type Primitive%20Component%20Object%20Reference) (bSelfMoved :type Boolean) (HitLocation :type Vector :default "0, 0, 0") (HitNormal :type Vector :default "0, 0, 0") (NormalImpulse :type Vector :default "0, 0, 0") (Hit :type Hit%20Result%20Structure%20%28by%20ref%29))
  ;[1 1 1] Check Collision
  (Variables|Default|Setcollision true))

(event EventTick
  (params (DeltaSeconds :type Float%20%28single-precision%29))
  (|CallParentFunction DeltaSeconds) ; This node is disabled and will not be called.\nDrag off pins to build functionality.
)

(event EventStep
  (params (Action :type Array%20of%20Floats%20%28double-precision%29))
  (bind _output (Utilities|Array|Get(acopy) Action 2))
  ;[1 1 1] Step
  (Math|Integer|IncrementInt (Variables|Default|GetCounter)
    (:%20%20
      (Development|PrintString (Utilities|String|ToString(Float) _output))
      (CallFunction|AddLateralMovement _output))))

(event Collision|EventActorBeginOverlap
  (params (OtherActor :type Actor%20Object%20Reference))
  (|CallParentFunction OtherActor) ; This node is disabled and will not be called.\nDrag off pins to build functionality.
)

(fn ConstructionScript
  (|CallParentFunction))

(fn GetAgentReward
  (if (Variables|Default|Getcollision)
    (Variables|Default|SetReward -1.0)
    (elif (Variables|Default|GetisKnownField)
      (Variables|Default|SetReward -0.5)
      (else
        (Variables|Default|SetReward 1.0))))
  (return (Variables|Default|GetReward)))

(fn ResetAgent
  (bind _returnvalue (Game|SpawnActorfromClass "/unray/Blueprints/MultiAgentArena/BP_ArenaAgent1.BP_ArenaAgent1_C" (Math|Transform|MakeTransform (Math|Vector|MakeVector 5e+01 7.5e+02 (.z (Transformation|GetActorLocation))) "0, 0, 0" "1.000000,1.000000,1.000000") "AlwaysSpawn" 0 0))
  (return _returnvalue))

(fn GetState
  (bind _pos (CallFunction|GetAgentState))
  (return _pos))

(fn GetAgentState
  (bind _returnvalue (Transformation|GetActorLocation))
  (bind _returnvalue_2 (Math|Float|Absolute(Float) (.x _returnvalue)))
  (bind _returnvalue_3 (Math|Float|Absolute(Float) (.y _returnvalue)))
  (bind _returnvalue_4 (- _returnvalue_2 5e+01))
  (bind _returnvalue_5 (- _returnvalue_3 5e+01))
  (bind _returnvalue_6 (Math|Float|SafeDivide _returnvalue_4 1e+02))
  (bind _returnvalue_7 (Math|Float|SafeDivide _returnvalue_5 1e+02))
  (bind _returnvalue_8 (* _returnvalue_7 8.0))
  (bind _returnvalue_9 (+ _returnvalue_6 _returnvalue_8))
  (Utilities|Array|Add (Variables|Default|GetVisited) _returnvalue_9)
  (Variables|Default|SetisKnownField (Utilities|Array|ContainsItem (Variables|Default|GetVisited) _returnvalue_9))
  (return (Utilities|Array|MakeArray _returnvalue_9)))

(fn IsDone
  (bind _isagentdone (CallFunction|IsAgentDone))
  (return _isagentdone))

(fn GetSelfActor
  (return self))

(fn Reset
  (bind _newactor (CallFunction|ResetAgent))
  (return _newactor true))

(fn GetReward
  (bind _agentreward (CallFunction|GetAgentReward))
  (return _agentreward))

(fn IsAgentDone
  (bind _isagentdone (|CallParentFunction))
  (return _isagentdone))