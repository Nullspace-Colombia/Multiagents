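; Base agent for a multi-agent arena, with step, state, reward, done and reset functions that suggest reinforcement learning.
; Step picks this agent's action by its action index, and it and Enhanced Input both drive fixed-size four-way teleport moves on XY within configurable limits.
; A step counter ends episodes at MaxFrames, and hits set a collision flag.
; GetAgentState and ResetAgent are empty stubs, while construction tints the cube with the agent's color.
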(event Custom|AddLateralMovement
  (params (Input :type Float%20%28double-precision%29))
  ;[0.5697 1 0.4631] Actions
  (CallFunction|CheckLimitsX)
  (CallFunction|CheckLimitsY)
  (if (and (== Input 0.0) (not (Variables|Default|GetIsOverLimitUp)))
    (Transformation|SetActorLocation (+ (Transformation|GetActorLocation) (Math|Vector|MakeVector 0.0 -1e+02 0.0)) false false)
    (elif (and (== Input 2.0) (not (Variables|Default|GetIsOverLimitDown)))
      (Transformation|SetActorLocation (+ (Transformation|GetActorLocation) (Math|Vector|MakeVector 0.0 1e+02 0.0)) false false)
      (elif (and (== Input 1.0) (not (Variables|Default|GetIsOverLimitRight)))
        (Transformation|SetActorLocation (+ (Transformation|GetActorLocation) (Math|Vector|MakeVector 1e+02 0.0 0.0)) false false)
        (elif (and (== Input 3.0) (not (Variables|Default|GetIsOverLimitLeft)))
          (Transformation|SetActorLocation (+ (Transformation|GetActorLocation) (Math|Vector|MakeVector -1e+02 0.0 0.0)) false false))))))

(event Custom|CheckLimitsY
  (bind _returnvalue (Transformation|GetActorLocation))
  ;[1 1 1] Check Limits
  (Math|Float|CompareFloat (+ (.y _returnvalue) 1e+02) (Variables|Default|GetYLimH)
    (:>
      (Variables|Default|SetIsOverLimitDown true))
    (:==
      (Variables|Default|SetIsOverLimitDown false :!label _label))
    (:<
      (goto _label)))
  (Math|Float|CompareFloat (+ (.y _returnvalue) -1e+02) (Variables|Default|GetYLimL)
    (:>
      (Variables|Default|SetIsOverLimitUp false :!label _label_2))
    (:==
      (goto _label_2))
    (:<
      (Variables|Default|SetIsOverLimitUp true))))

(event Custom|CheckLimitsX
  (bind _returnvalue (Transformation|GetActorLocation))
  ;[1 1 1] Check Limits
  (Math|Float|CompareFloat (+ (.x _returnvalue) 1e+02) (Variables|Default|GetXLimH)
    (:>
      (Variables|Default|SetIsOverLimitRight true))
    (:==
      (Variables|Default|SetIsOverLimitRight false :!label _label))
    (:<
      (goto _label)))
  (Math|Float|CompareFloat (+ (.x _returnvalue) -1e+02) (Variables|Default|GetXLimL)
    (:>
      (Variables|Default|SetIsOverLimitLeft false :!label _label_2))
    (:==
      (goto _label_2))
    (:<
      (Variables|Default|SetIsOverLimitLeft true))))

(event Input|EnhancedActionEvents|EnhancedInputActionIA_MoveLeft
  (params (ActionValue :type Boolean) (ElapsedSeconds :type Float%20%28double-precision%29) (TriggeredSeconds :type Float%20%28double-precision%29) (InputAction :type Input%20Action%20Object%20Reference :default "/Game/Inputs/IA_MoveLeft.IA_MoveLeft"))
  ;[0.5697 1 0.4631] Actions
  (:Triggered
    (CallFunction|AddLateralMovement 3.0)))

(event Input|EnhancedActionEvents|EnhancedInputActionIA_MoveRight
  (params (ActionValue :type Boolean) (ElapsedSeconds :type Float%20%28double-precision%29) (TriggeredSeconds :type Float%20%28double-precision%29) (InputAction :type Input%20Action%20Object%20Reference :default "/Game/Inputs/IA_MoveRight.IA_MoveRight"))
  ;[0.5697 1 0.4631] Actions
  (:Triggered
    (CallFunction|AddLateralMovement 1.0)))

(event Input|EnhancedActionEvents|EnhancedInputActionIA_MoveDown
  (params (ActionValue :type Boolean) (ElapsedSeconds :type Float%20%28double-precision%29) (TriggeredSeconds :type Float%20%28double-precision%29) (InputAction :type Input%20Action%20Object%20Reference :default "/Game/Inputs/IA_MoveDown.IA_MoveDown"))
  ;[0.5697 1 0.4631] Actions
  (:Triggered
    (CallFunction|AddLateralMovement 2.0)))

(event Input|EnhancedActionEvents|EnhancedInputActionIA_MoveUp
  (params (ActionValue :type Boolean) (ElapsedSeconds :type Float%20%28double-precision%29) (TriggeredSeconds :type Float%20%28double-precision%29) (InputAction :type Input%20Action%20Object%20Reference :default "/Game/Inputs/IA_MoveUp.IA_MoveUp"))
  ;[0.5697 1 0.4631] Actions
  (:Triggered
    (CallFunction|AddLateralMovement 0.0)))

(event EventBeginPlay
  ;[1 1 1] Initial Configuration
  (bind _asplayer_controller (Utilities|Casting|CastToPlayerController (Pawn|GetController)))
  (Utilities|IsValid (PlayerController|LocalPlayerSubsystems|GetEnhancedInputLocalPlayerSubsystem _asplayer_controller)
    (:Is%20Valid
      (Input|AddMappingContext (PlayerController|LocalPlayerSubsystems|GetEnhancedInputLocalPlayerSubsystem _asplayer_controller) "/Game/Inputs/IMC_Arena.IMC_Arena" 0 "(bIgnoreAllPressedKeysUntilRelease=True,bForceImmediately=False)")
      (Pawn|Components|CharacterMovement|SetMovementMode (Variables|Character|GetCharacterMovement) "MOVE_Flying" 0))))

(event Collision|EventHit
  (params (MyComp :type Primitive%20Component%20Object%20Reference) (Other :type Actor%20Object%20Reference) (OtherComp :type Primitive%20Component%20Object%20Reference) (bSelfMoved :type Boolean) (HitLocation :type Vector :default "0, 0, 0") (HitNormal :type Vector :default "0, 0, 0") (NormalImpulse :type Vector :default "0, 0, 0") (Hit :type Hit%20Result%20Structure%20%28by%20ref%29))
  ;[1 1 1] Check Collision
  (Variables|Default|Setcollision true))

(event EventTick
  (params (DeltaSeconds :type Float%20%28single-precision%29)))

(event Collision|EventActorBeginOverlap
  (params (OtherActor :type Actor%20Object%20Reference)))

(event EventStep
  (params (Action :type Array%20of%20Floats%20%28double-precision%29))
  ;[1 1 1] Step
  (Math|Integer|IncrementInt (Variables|Default|GetCounter)
    (:%20%20
      (CallFunction|AddLateralMovement (Utilities|Array|Get(acopy) Action (Variables|Default|Getaction))))))

(event EventSetID
  (params (ID :type Integer))
  (Variables|Default|SetID ID))

(event EventSetActionID
  (params (ActionID :type Integer))
  (Variables|Default|Setaction ActionID))

(fn ConstructionScript
  (bind _returnvalue (Rendering|Material|CreateDynamicMaterialInstance (Variables|Default|GetCube) 0 0 "None" :!class /Script/Engine.PrimitiveComponent))
  (Rendering|Material|SetVectorParameterValue _returnvalue "Param" (Variables|Default|GetColor) :!class /Script/Engine.MaterialInstanceDynamic))

(fn GetAgentState
  (return 0))

(fn GetAgentReward
  (return (Variables|Default|GetReward)))

(fn IsAgentDone
  (Math|Integer|CompareInt (Variables|Default|GetCounter) (Variables|Default|GetMaxFrames)
    (:>
      (Variables|Default|SetDone true :!label _label)
      (Variables|Default|SetCounter 0))
    (:==
      (goto _label))
    (:<
      (Variables|Default|SetDone false)))
  (return (Variables|Default|GetDone)))

(fn ResetAgent
  (return 0))

(fn SetLimits
  (params (LImXH :type Float%20%28double-precision%29) (LimXL :type Float%20%28double-precision%29) (LimYH :type Float%20%28double-precision%29) (LimYL :type Float%20%28double-precision%29) (OffsetX :type Float%20%28double-precision%29) (OffsetY :type Float%20%28double-precision%29))
  (Variables|Default|SetXLimH LImXH)
  (Variables|Default|SetXLimL LimXL)
  (Variables|Default|SetYLimH LimYH)
  (Variables|Default|SetYLimL LimYL)
  (Variables|Default|SetOffsetX OffsetX)
  (Variables|Default|SetOffsetY OffsetY))

(fn GetID
  (return (Variables|Default|GetID)))

(fn GetReward
  (bind _agentreward (CallFunction|GetAgentReward))
  (return _agentreward))

(fn GetSelfActor
  (return self))

(fn GetState
  (bind _pos (CallFunction|GetAgentState))
  (return _pos))

(fn IsDone
  (bind _isagentdone (CallFunction|IsAgentDone))
  (return _isagentdone))

(fn Reset
  (bind _newactor (CallFunction|ResetAgent))
  (return _newactor true))