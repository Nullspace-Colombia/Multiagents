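; BP_ArenaAgent2 is a reinforcement-learning agent in the multi-agent arena, exposing step, state, reward, done and reset functions.
; Each step applies the action as lateral movement, and state flattens its offset-relative position into an eight-wide grid index, logging visited cells.
; A hit sets a collision flag, never cleared here, that turns the small negative reward positive.
; Reset teleports it to a fixed offset position; termination defers to the parent.
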(event EventBeginPlay
  (|CallParentFunction) ; This node is disabled and will not be called.\nDrag off pins to build functionality.
)

(event Collision|EventHit
  (params (MyComp :type Primitive%20Component%20Object%20Reference) (Other :type Actor%20Object%20Reference) (OtherComp :type Primitive%20Component%20Object%20Reference) (bSelfMoved :type Boolean) (HitLocation :type Vector :default "0, 0, 0") (HitNormal :type Vector :default "0, 0, 0") (NormalImpulse :type Vector :default "0, 0, 0") (Hit :type Hit%20Result%20Structure%20%28by%20ref%29))
  ;[1 1 1] Check Collision
  (Variables|Default|Setcollision true))

(event EventTick
  (params (DeltaSeconds :type Float%20%28single-precision%29))
  (|CallParentFunction DeltaSeconds) ; This node is disabled and will not be called.\nDrag off pins to build functionality.
)

(event EventStep
  (params (Action :type Array%20of%20Floats%20%28double-precision%29))
  ;[1 1 1] Step
  (Math|Integer|IncrementInt (Variables|Default|GetCounter)
    (:%20%20
      (CallFunction|AddLateralMovement (Utilities|Array|Get(acopy) Action (Variables|Default|Getaction))))))

(event Collision|EventActorBeginOverlap
  (params (OtherActor :type Actor%20Object%20Reference))
  (|CallParentFunction OtherActor) ; This node is disabled and will not be called.\nDrag off pins to build functionality.
)

(fn ConstructionScript
  (|CallParentFunction))

(fn GetAgentReward
  (if (Variables|Default|Getcollision)
    (Variables|Default|SetReward 1.0)
    (else
      (Variables|Default|SetReward -0.1)))
  (return (Variables|Default|GetReward)))

(fn ResetAgent
  (Transformation|SetActorLocation (Math|Vector|MakeVector (+ (Variables|Default|GetOffsetX) 7e+02) (+ (Variables|Default|GetOffsetY) 7e+02) (.z (Transformation|GetActorLocation))) false true)
  (return self))

(fn GetState
  (bind _returnvalue (Transformation|GetActorLocation))
  (bind _offsetx (Variables|Default|GetOffsetX))
  (bind _offsety (Variables|Default|GetOffsetY))
  (bind _returnvalue_2 (- (.y _returnvalue) _offsety))
  (bind _returnvalue_3 (- (.x _returnvalue) _offsetx))
  (bind _returnvalue_4 (Math|Float|Absolute(Float) _returnvalue_3))
  (bind _returnvalue_5 (Math|Float|Absolute(Float) _returnvalue_2))
  (bind _returnvalue_6 (Math|Float|SafeDivide _returnvalue_4 1e+02))
  (bind _returnvalue_7 (Math|Float|SafeDivide _returnvalue_5 1e+02))
  (bind _returnvalue_8 (* _returnvalue_7 8.0))
  (bind _returnvalue_9 (+ _returnvalue_6 _returnvalue_8))
  (Utilities|Array|Add (Variables|Default|GetVisited) _returnvalue_9)
  (Variables|Default|SetisKnownField (Utilities|Array|ContainsItem (Variables|Default|GetVisited) _returnvalue_9))
  (return (Utilities|Array|MakeArray _returnvalue_9)))

(fn GetAgentState
  (bind _pos (CallFunction|GetAgentState))
  (return _pos))

(fn IsDone
  (bind _isagentdone (CallFunction|IsAgentDone))
  (return _isagentdone))

(fn GetSelfActor
  (return self))

(fn Reset
  (bind _newactor (CallFunction|ResetAgent))
  (return _newactor false))

(fn GetReward
  (bind _agentreward (CallFunction|GetAgentReward))
  (return _agentreward))

(fn IsAgentDone
  (bind _isagentdone (|CallParentFunction))
  (return _isagentdone))