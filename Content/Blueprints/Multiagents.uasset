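; Test Blueprint for a multi-agent reinforcement-learning bridge that runs a local server and exchanges agent data with an external client.
; Tick services the connection and, once connected, sends three hardcoded agents with differing observation counts, optionally including reward and done state.
; A Gate keeps the exchange in lockstep: it closes after each send and reopens when received data yields actions, which are printed on screen.
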(event Custom|OnDataReceptionDelegate_Event
  (params (Arr :type Array%20of%20Bytes))
  (bind _returnvalue (Class|Pole|GetAction Arr))
  (for _array_element _returnvalue
    (Development|PrintString (Utilities|String|ToString(Float) _array_element) true true "(R=0.000000,G=0.660000,B=1.000000,A=1.000000)" 1e+01)
    (CallFunction|OpenGate)))

(event Custom|Close_Gate
  (Utilities|FlowControl|Gate false) ; enters at Close
)

(event Custom|Open_Gate
  (Utilities|FlowControl|Gate false) ; enters at Open
)

(event EventBeginPlay
  (EventDispatchers|AssignOnDataReceptionDelegate (delegate Custom|OnDataReceptionDelegate_Event))
  (Class|Pole|StartServer "127.0.0.1" 10010))

(event EventTick
  (params (DeltaSeconds :type Float%20%28single-precision%29))
  (Class|Pole|ConductConnection)
  (if (Variables|Default|Getconnected)
    (Utilities|FlowControl|Gate false
      (:Exit
        (bind _returnvalue (Class|Pole|AddAgent 1 (Utilities|Array|MakeArray 1.5 2.36 4.58 -3.25) 0.0 false))
        (bind _returnvalue_2 (Class|Pole|AddAgent 2 (Utilities|Array|MakeArray 5.0 4.0 2e+01 2.36 0.0) 0.0 false))
        (bind _returnvalue_3 (Class|Pole|AddAgent 3 (Utilities|Array|MakeArray 5.0 4.0 2e+01 2.36 0.0 1.25) 1.0 true))
        (Class|Pole|SendMultiagentsInfo (Class|Pole|GetAgentsInfo _returnvalue _returnvalue_2 _returnvalue_3))
        (CallFunction|CloseGate)))))

(fn ConstructionScript)