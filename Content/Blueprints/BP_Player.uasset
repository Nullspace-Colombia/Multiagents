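; BP_Player is a player Blueprint that pushes a static mesh sideways with physics forces.
; Enhanced Input actions for left and right each print a debug string and apply a Y-axis force scaled by ForwardForce and a Left or Right variable.
; BeginPlay applies a single small roll rotation to the Cube component, while Tick and the construction script are empty.
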(event Input|EnhancedActionEvents|EnhancedInputActionIA_cube_left
  (params (ActionValue :type Boolean) (ElapsedSeconds :type Float%20%28double-precision%29) (TriggeredSeconds :type Float%20%28double-precision%29) (InputAction :type Input%20Action%20Object%20Reference :default "/Game/IA_cube_left.IA_cube_left"))
  (:Triggered
    (Development|PrintString "left")
    ;[0 0 0] Move Left
    (Physics|AddForce (Variables|Debug|GetStaticMeshComponent) (* (Math|Vector|MakeVector 0.0 (* 1e+03 (Variables|Movement|GetForward%20Force)) 0.0) (Variables|Default|Getleft)) "None" false)))

(event Input|EnhancedActionEvents|EnhancedInputActionIA_cube_right
  (params (ActionValue :type Boolean) (ElapsedSeconds :type Float%20%28double-precision%29) (TriggeredSeconds :type Float%20%28double-precision%29) (InputAction :type Input%20Action%20Object%20Reference :default "/Game/IA_cube_right.IA_cube_right"))
  (:Triggered
    (Development|PrintString "right")
    ;[0 0 0] Move Right
    (Physics|AddForce (Variables|Debug|GetStaticMeshComponent) (* (Math|Vector|MakeVector 0.0 (* 1e+03 (Variables|Movement|GetForward%20Force)) 0.0) (Variables|Default|Getright)) "None" false)))

(event EventBeginPlay
  (Transformation|AddWorldRotation (Variables|Default|GetCube) "0.000000,0.000000,5.000000" false false))

(event EventTick
  (params (DeltaSeconds :type Float%20%28single-precision%29)))

(fn ConstructionScript)