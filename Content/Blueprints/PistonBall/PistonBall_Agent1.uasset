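; PistonBall_Agent1 is a child agent Blueprint for the PistonBall environment, adding no behavior of its own.
; Its Step, Move, SetActionID and SetID events only forward their arguments to the parent class, as does the construction script.
; GetState is an empty stub, and the BeginPlay, overlap and Tick events are disabled placeholders.
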(event EventBeginPlay)

(event Collision|EventActorBeginOverlap
  (params (OtherActor :type Actor%20Object%20Reference))
  (|CallParentFunction OtherActor) ; This node is disabled and will not be called.\nDrag off pins to build functionality.
)

(event EventTick
  (params (DeltaSeconds :type Float%20%28single-precision%29)))

(event EventStep
  (params (Action :type Array%20of%20Floats%20%28double-precision%29))
  (|CallParentFunction Action))

(event EventMove
  (params (NewParam :type Float%20%28double-precision%29))
  (|CallParentFunction NewParam))

(event EventSetActionID
  (params (ActionID :type Integer))
  (|CallParentFunction ActionID))

(event EventSetID
  (params (ID :type Integer))
  (|CallParentFunction ID))

(fn ConstructionScript
  (|CallParentFunction))

(fn GetState)