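; PistonBallArena is an arena actor for a piston-ball agent setup, with plane, ball and child-actor agent components.
; BeginPlay only loops the root's child components, compares each to the first BaseAgentPistonBall found and prints matches.
; Disconnected setup logic would collect agents, attach and position them in a row, reset them, place the ball and tint materials, but never runs.
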(event EventBeginPlay
  (for _array_element (Components|GetChildrenComponents (Variables|Default|GetDefaultSceneRoot) false)
    (bind _returnvalue (Actor|GetActorOfClass "/Game/Blueprints/PistonBall/BaseAgentPistonBall.BaseAgentPistonBall_C"))
    (if (== _returnvalue _array_element)
      (Development|PrintString (Utilities|GetDisplayName _array_element)))))

(event Collision|EventActorBeginOverlap
  (params (OtherActor :type Actor%20Object%20Reference)))

(event EventTick
  (params (DeltaSeconds :type Float%20%28single-precision%29)))

(fn ConstructionScript)