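; Base piston agent for a PistonBall multi-agent environment, apparently for reinforcement learning, exposing step, state, reward, done and reset functions.
; Step picks this agent's entry from the action array and slides the Body between raised and lowered heights.
; State is the capsule's relative Z, while reward and done are constant placeholders.
; Reset randomizes the Body height, and construction tints Body and Head through dynamic materials.
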(event EventMove
  (params (NewParam :type Float%20%28double-precision%29))
  (bind _body (Variables|Default|GetBody))
  (bind _relativelocation (Variables|/Script/Engine.SceneComponent|GetRelativeLocation _body))
  ;[1 1 1] movement
  (Math|Integer|IncrementInt (Variables|Default|GetCounter)
    (:%20%20
      (if (== NewParam 0.0)
        (Components|MoveComponentTo _body (Math|Vector|MakeVector (.x _relativelocation) (.y _relativelocation) 1e+02) "0, 0, 0" false false 0.08 false)
        (elif (== NewParam 1.0)
          (Components|MoveComponentTo _body (Math|Vector|MakeVector (.x _relativelocation) (.y _relativelocation) 0.0) "0, 0, 0" false false 0.08 false))))))

(event EventSetActionID
  (params (ActionID :type Integer))
  (Variables|Default|SetAction ActionID))

(event EventSetID
  (params (ID :type Integer))
  (Variables|Default|SetID ID))

(event Collision|EventActorBeginOverlap
  (params (OtherActor :type Actor%20Object%20Reference)))

(event EventStep
  (params (Action :type Array%20of%20Floats%20%28double-precision%29))
  ;[1 1 1] Step
  (CallFunction|Move (Utilities|Array|Get(acopy) Action (Variables|Default|GetAction))))

(fn ConstructionScript
  (bind _returnvalue (Rendering|Material|CreateDynamicMaterialInstance (Variables|Default|GetBody) 0 "/Game/Materials/MultiAgentArena.MultiAgentArena" "None" :!class /Script/Engine.PrimitiveComponent))
  (Rendering|Material|SetVectorParameterValue _returnvalue "Param" (Variables|Default|GetColor_Body) :!class /Script/Engine.MaterialInstanceDynamic)
  (bind _returnvalue_2 (Rendering|Material|CreateDynamicMaterialInstance (Variables|Default|GetHead) 0 "/Game/Materials/MultiAgentArena.MultiAgentArena" "None" :!class /Script/Engine.PrimitiveComponent))
  (Rendering|Material|SetVectorParameterValue _returnvalue_2 "Param" (Variables|Default|GetColor_Head) :!class /Script/Engine.MaterialInstanceDynamic))

(fn GetAgentState
  (return (Utilities|Array|MakeArray (.z (Variables|/Script/Engine.SceneComponent|GetRelativeLocation (Variables|Collision|GetCapsuleComponent))))))

(fn GetAgentReward
  (return 0.0))

(fn IsAgentDone
  (return false))

(fn GetID
  (return (Variables|Default|GetID)))

(fn GetReward
  (bind _agentreward (CallFunction|GetAgentReward))
  (return _agentreward))

(fn GetSelfActor
  (return self))

(fn GetState
  (bind _pos (CallFunction|GetAgentState))
  (return _pos))

(fn IsDone
  (bind _isagentdone (CallFunction|IsAgentDone))
  (return _isagentdone))

(fn Reset
  (bind _body (Variables|Default|GetBody))
  (bind _relativelocation (Variables|/Script/Engine.SceneComponent|GetRelativeLocation _body))
  (Transformation|SetRelativeLocation _body (Math|Vector|MakeVector (.x _relativelocation) (.y _relativelocation) (.OutItem (Utilities|Array|Random (Utilities|Array|MakeArray 0.0 1e+02)))) false false)
  (Variables|Default|SetDone false)
  (return 0 false))