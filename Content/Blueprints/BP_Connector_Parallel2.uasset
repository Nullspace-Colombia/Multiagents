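; Multi-agent reinforcement learning connector that links agents from every MultiAgent_Env arena to an external client through a local socket server.
; On BeginPlay it gathers agents, assigns arena-based IDs, starts the server and sets time dilation.
; Tick services the connection; received actions open a gate for one Step, which applies them, resets or replaces finished agents, and returns observations, rewards and done flags.
; Several alternative step implementations remain unwired.
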(event Custom|SetAgents
  ;[1 1 1] SetAgents
  (bind _outactors (Actor|GetAllActorsOfClass "/Game/Blueprints/MultiAgentArena/MultiAgent_Env.MultiAgent_Env_C"))
  (for (_array_element _array_index) _outactors
    (bind _asmulti_agent_env (Utilities|Casting|CastToMultiAgent_Env _array_element))
    (for (_array_element_2 _array_index_2) (Variables|/Game/Blueprints/MultiAgentArena/MultiAgent_Env.MultiAgent_Env_C|GetAgents _asmulti_agent_env)
      (bind _asbi_agent (Utilities|Casting|CastToBI_Agent _array_element_2))
      (Utilities|Array|Add (Variables|Default|GetAgents) _asbi_agent)
      (bind _agentid (CallFunction|SetAgentID _array_index _array_index_2))
      (Default|SetID _asbi_agent _agentid)
      (Default|SetActionID _asbi_agent (- _agentid (Math|Float|Truncate (* (Variables|Default|Getenv_id) 1e+01))))))
  (for _array_element_3 (Variables|Default|GetAgents)
    (bind _id (Default|GetID _array_element_3))
    (Development|PrintString (Utilities|String|ToString(Integer) _id))))

(event Custom|SendAgents
  ;[1 1 1] Send Angents Info
  (Class|Pole|SendMultiagentsInfo (Variables|Default|GetAgentsInfo))
  (Utilities|Array|Clear (Variables|Default|GetAgentsInfo)))

(event Custom|CheckAllDone
  ;[1 0.5425 0.5047] Check if all agents are done
  (for _array_element (Variables|Default|GetIsDone_Agents)
    (if _array_element
      (Math|Integer|IncrementInt (Variables|Default|GetAgentsDone))))
  (Math|Integer|CompareInt (Variables|Default|GetAgentsDone) (Utilities|Array|Length (Variables|Default|GetAgents))
    (:==
      (Variables|Default|SetIsDoneTotal true))
    (:<
      (Variables|Default|SetIsDoneTotal false))))

(event Custom|CheckIsDone
  ;[1 0.7462 0.2384] Check Done
  (for _array_element (Variables|Default|GetAgents)
    (bind _bdone (Default|IsDone _array_element))
    (Utilities|Array|Add (Variables|Default|GetIsDone_Agents) _bdone)
    (bind _reward (Default|GetReward _array_element))
    (Utilities|Array|Add (Variables|Default|GetRewards) _reward)))

(event Custom|StartConnection
  ;[0.4158 0.6112 1] Start Connection
  (|SyncData)
  (Class|Pole|StartServer "127.0.0.1" 10011))

(event Custom|GetInfo
  (params (Agent :type BI%20Agent%20Interface) (Index :type Integer))
  ;[0.6448 1 0.6882] Step
  (bind _observations (Default|GetState Agent))
  (bind _reward (Default|GetReward Agent))
  (bind _bdone (Default|IsDone Agent))
  (bind _id (Default|GetID Agent))
  (Utilities|Array|SetArrayElem (Variables|Default|GetIsDone_Agents) Index _bdone)
  (if _bdone
    (bind (_newactor _bcreateactor) (Default|Reset Agent))
    (if _bcreateactor
      (bind _actor (Default|GetSelfActor _newactor))
      (Actor|DestroyActor _actor)
      (Utilities|Array|SetArrayElem (Variables|Default|GetAgents) Index _newactor))
    (bind _observations_2 (Default|GetState _newactor))
    (bind _returnvalue (Class|Pole|AddAgent _id _observations_2 _reward _bdone))
    (Utilities|Array|AppendArray (Variables|Default|GetAgentsInfo) _returnvalue)
    (else
      (bind _returnvalue_2 (Class|Pole|AddAgent _id _observations _reward _bdone))
      (Utilities|Array|AppendArray (Variables|Default|GetAgentsInfo) _returnvalue_2))))

(event Custom|Step
  (bind _isdone_agents (Variables|Default|GetIsDone_Agents))
  ;[0.6448 1 0.6882] Step
  (CallFunction|CloseGate)
  (if (Variables|Default|Getinitial_state)
    (for (_array_element _array_index) (Variables|Default|GetAgents)
      (CallFunction|GetInfo _array_element _array_index))
    (CallFunction|SendAgents)
    (Variables|Default|Setinitial_state false)
    (Development|PrintString "Initial Obs" true false)
    (else
      (if (Variables|Default|GetIsDoneTotal)
        (for (_ _array_index_2) _isdone_agents
          (Utilities|Array|SetArrayElem _isdone_agents _array_index_2 false)))
      (for (_array_element_2 _array_index_3) (Variables|Default|GetAgents)
        (if (Utilities|Array|Get(acopy) (Variables|Default|GetIsDone_Agents) _array_index_3)
          (Utilities|Array|Insert (Variables|Default|GetActions) 0.0)
          (else
            (Default|Step _array_element_2 (Variables|Default|GetActions)))))
      (for (_array_element_3 _array_index_4) (Variables|Default|GetAgents)
        (CallFunction|GetInfo _array_element_3 _array_index_4))
      (CallFunction|SendAgents)
      (Variables|Default|SetIsDoneTotal true)
      (for _array_element_4 (Variables|Default|GetIsDone_Agents)
        (Variables|Default|SetIsDoneTotal (and _array_element_4 (Variables|Default|GetIsDoneTotal)))))))

(event EventTick
  (params (DeltaSeconds :type Float%20%28single-precision%29))
  (CallFunction|Hop))

(event EventBeginPlay
  (CallFunction|SetAgents)
  (CallFunction|StartConnection)
  (Utilities|Time|SetGlobalTimeDilation (Variables|Default|GetTime%20Dilation))
  (Variables|Default|Setinitial_state true))

(fn ConstructionScript)

(fn SetAgentID
  (params (ArenaID :type Integer) (Agent :type Integer))
  (return (Math|Conversions|ToInteger(Byte) (Utilities|String|Append (Utilities|String|ToString(Integer) (+ ArenaID 1)) (Utilities|String|ToString(Integer) (+ Agent 1))))))

(event Custom|Open_Gate
  (Utilities|FlowControl|Gate true) ; enters at Open
)

(event Custom|Close_Gate
  (Utilities|FlowControl|Gate true) ; enters at Close
)

(event Custom|Hop
  (Class|Pole|ConductConnection)
  (if (Variables|Default|Getconnected)
    (Utilities|FlowControl|Gate true
      (:Exit
        (CallFunction|Step)))))

(event Custom|OnDataReceptionDelegate_Event_0
  (params (Arr :type Array%20of%20Bytes))
  (bind _returnvalue (Class|Pole|GetAction Arr))
  (bind _output_get (Variables|Default|SetActions _returnvalue))
  (Variables|Default|Setenv_id (Utilities|Array|Get(acopy) _output_get))
  (CallFunction|OpenGate))