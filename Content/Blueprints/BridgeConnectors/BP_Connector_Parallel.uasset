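; Bridge connector that links parallel multi-agent environments to an external client through a local server, apparently for reinforcement learning, under adjustable time dilation.
; On BeginPlay it gathers agents from every MultiAgent_Env and assigns arena-based IDs and action IDs.
; Tick services the connection, with a gate keeping steps in lockstep with received actions.
; Each step resets finished agents, steps the others, and returns observations, rewards and done flags.
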(event Custom|SetAgents
  ;[1 1 1] SetAgents
  (bind _outactors (Actor|GetAllActorsOfClass "/Game/Blueprints/MultiAgentArena/MultiAgent_Env.MultiAgent_Env_C"))
  (for (_array_element _array_index) _outactors
    (bind _asmulti_agent_env (Utilities|Casting|CastToMultiAgent_Env _array_element))
    (for (_array_element_2 _array_index_2) (Variables|/Game/Blueprints/MultiAgentArena/MultiAgent_Env.MultiAgent_Env_C|GetAgents _asmulti_agent_env)
      (bind _asbi_agent (Utilities|Casting|CastToBI_Agent _array_element_2))
      (Utilities|Array|Add (Variables|Default|GetAgents) _asbi_agent)
      (bind _agentid (CallFunction|SetAgentID _array_index _array_index_2))
      (Default|SetID _asbi_agent _agentid)
      (bind _result (Math|Integer|IncrementInt (Variables|Default|GetactionID))
        (:%20%20
          (Default|SetActionID _asbi_agent _result)))))
  (for _array_element_3 (Variables|Default|GetAgents)
    (bind _id (Default|GetID _array_element_3))
    (Development|PrintString (Utilities|String|ToString(Integer) _id))))

(event Custom|SendAgents
  ;[1 1 1] Send Angents Info
  (Class|Pole|SendMultiagentsInfo (Variables|Default|GetAgentsInfo))
  (Utilities|Array|Clear (Variables|Default|GetAgentsInfo)))

(event Custom|CheckAllDone
  ;[1 0.5425 0.5047] Check if all agents are done
  (for _array_element (Variables|Default|GetIsDone_Agents)
    (if _array_element
      (Math|Integer|IncrementInt (Variables|Default|GetAgentsDone))))
  (Math|Integer|CompareInt (Variables|Default|GetAgentsDone) (Utilities|Array|Length (Variables|Default|GetAgents))
    (:==
      (Variables|Default|SetIsDoneTotal true))
    (:<
      (Variables|Default|SetIsDoneTotal false))))

(event Custom|CheckIsDone
  ;[1 0.7462 0.2384] Check Done
  (for _array_element (Variables|Default|GetAgents)
    (bind _bdone (Default|IsDone _array_element))
    (Utilities|Array|Add (Variables|Default|GetIsDone_Agents) _bdone)
    (bind _reward (Default|GetReward _array_element))
    (Utilities|Array|Add (Variables|Default|GetRewards) _reward)))

(event Custom|StartConnection
  ;[0.4158 0.6112 1] Start Connection
  (|SyncData)
  (Class|Pole|StartServer "127.0.0.1" 10011))

(event Custom|Step
  ;[0.6156 1 0.6535] Possible Multiagent Step
  (CallFunction|CheckAllDone)
  (if (Variables|Default|GetIsDoneTotal)
    (for (_array_element _array_index) (Variables|Default|GetAgents)
      (bind (_newactor _bcreateactor) (Default|Reset _array_element))
      (if _bcreateactor
        (bind _actor (Default|GetSelfActor _array_element))
        (Actor|DestroyActor _actor)
        (Utilities|Array|SetArrayElem (Variables|Default|GetAgents) _array_index _newactor))
      (bind _observations (Default|GetState _newactor))
      (bind _id (Default|GetID _newactor))
      (bind _returnvalue (Class|Pole|AddAgent _id _observations (Utilities|Array|Get(acopy) (Variables|Default|GetRewards) _array_index) (Utilities|Array|Get(acopy) (Variables|Default|GetIsDone_Agents) _array_index)))
      (Utilities|Array|AppendArray (Variables|Default|GetAgentsInfo) _returnvalue))
    (CallFunction|SendAgents)
    (Variables|Default|SetIsDoneTotal false)
    (CallFunction|CloseGate)
    (else
      (Utilities|Array|Clear (Variables|Default|GetIsDone_Agents))
      (Utilities|Array|Clear (Variables|Default|GetRewards))
      (CallFunction|CheckIsDone)
      (for (_array_element_2 _array_index_2) (Variables|Default|GetAgents)
        (if (Utilities|Array|Get(acopy) (Variables|Default|GetIsDone_Agents) _array_index_2)
          (bind (_newactor_2 _bcreateactor_2) (Default|Reset _array_element_2))
          (if _bcreateactor_2
            (bind _actor_2 (Default|GetSelfActor _array_element_2))
            (Actor|DestroyActor _actor_2)
            (Utilities|Array|SetArrayElem (Variables|Default|GetAgents) _array_index_2 _newactor_2))
          (bind _observations_2 (Default|GetState _newactor_2))
          (bind _id_2 (Default|GetID _newactor_2))
          (bind _returnvalue_2 (Class|Pole|AddAgent _id_2 _observations_2 (Utilities|Array|Get(acopy) (Variables|Default|GetRewards) _array_index_2) (Utilities|Array|Get(acopy) (Variables|Default|GetIsDone_Agents) _array_index_2)))
          (Utilities|Array|AppendArray (Variables|Default|GetAgentsInfo) _returnvalue_2)
          (else
            (Default|Step _array_element_2 (Variables|Default|GetActions))
            (bind _observations_3 (Default|GetState _array_element_2))
            (bind _id_3 (Default|GetID _array_element_2))
            (bind _returnvalue_3 (Class|Pole|AddAgent _id_3 _observations_3 (Utilities|Array|Get(acopy) (Variables|Default|GetRewards) _array_index_2) (Utilities|Array|Get(acopy) (Variables|Default|GetIsDone_Agents) _array_index_2)))
            (Utilities|Array|AppendArray (Variables|Default|GetAgentsInfo) _returnvalue_3))))
      (CallFunction|SendAgents)
      (CallFunction|CloseGate))))

(event EventTick
  (params (DeltaSeconds :type Float%20%28single-precision%29))
  (CallFunction|Hop))

(event EventBeginPlay
  (CallFunction|SetAgents)
  (CallFunction|StartConnection)
  (Utilities|Time|SetGlobalTimeDilation (Variables|Default|GetTime%20Dilation)))

(fn ConstructionScript)

(fn SetAgentID
  (params (ArenaID :type Integer) (Agent :type Integer))
  (return (Math|Conversions|ToInteger(Byte) (Utilities|String|Append (Utilities|String|ToString(Integer) (+ ArenaID 1)) (Utilities|String|ToString(Integer) (+ Agent 1))))))

(event Custom|Open_Gate
  (Utilities|FlowControl|Gate false) ; enters at Open
)

(event Custom|Close_Gate
  (Utilities|FlowControl|Gate false) ; enters at Close
)

(event Custom|Hop
  (Class|Pole|ConductConnection)
  (if (Variables|Default|Getconnected)
    (Utilities|FlowControl|Gate false
      (:Exit
        (CallFunction|Step)))))

(event Custom|OnDataReceptionDelegate_Event_0
  (params (Arr :type Array%20of%20Bytes))
  (bind _returnvalue (Class|Pole|GetAction Arr))
  (Variables|Default|SetActions _returnvalue)
  (CallFunction|OpenGate))