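; BP_Connector links an agent actor implementing BI_Agent to an external client through a local socket server, in a reinforcement-learning style loop.
; Received data becomes actions and opens a gate, so a connected Tick runs one Step, returns observations, reward and done, then closes the gate.
; Finished episodes reset the agent, replacing its actor when requested, instead of applying actions.
; Global time dilation sets simulation speed.
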(event Custom|CheckIsDone
  (bind _agent (Variables|Default|GetAgent))
  ;[1 0.7462 0.2384] Check Done
  (bind _bdone (Default|IsDone _agent))
  (Variables|Default|SetIsDone _bdone)
  (bind _reward (Default|GetReward _agent))
  (Variables|Default|SetReward _reward))

(event Custom|StartConnection
  ;[0.4158 0.6112 1] Start Connection
  (|SyncData)
  (Class|Pole|StartServer "127.0.0.1" 10010))

(event Custom|Step
  ;[0.331 1 0.3281] Step
  (CallFunction|CheckIsDone)
  (if (Variables|Default|GetIsDone)
    (bind (_newactor _bcreateactor) (Default|Reset (Variables|Default|GetAgent)))
    (if _bcreateactor
      (bind _actor (Default|GetSelfActor (Variables|Default|GetAgent)))
      (Actor|DestroyActor _actor)
      (Variables|Default|SetAgent _newactor))
    (bind _observations (Default|GetState (Variables|Default|GetAgent)))
    (Class|Pole|SendState _observations (Variables|Default|GetReward) (Variables|Default|GetIsDone))
    (CallFunction|CloseGate)
    (else
      (Default|Step (Variables|Default|GetAgent) (Variables|Default|GetActions))
      (bind _observations_2 (Default|GetState (Variables|Default|GetAgent)))
      (Class|Pole|SendState _observations_2 (Variables|Default|GetReward) (Variables|Default|GetIsDone))
      (CallFunction|CloseGate))))

(event EventTick
  (params (DeltaSeconds :type Float%20%28single-precision%29))
  (CallFunction|Hop))

(event EventBeginPlay
  (bind _asbi_agent (Utilities|Casting|CastToBI_Agent (Variables|Default|GetActorAgent)))
  (Variables|Default|SetAgent _asbi_agent)
  (CallFunction|StartConnection)
  (Utilities|Time|SetGlobalTimeDilation (Variables|Default|GetTime%20Dilation)))

(fn ConstructionScript)

(event Custom|Open_Gate
  (Utilities|FlowControl|Gate false) ; enters at Open
)

(event Custom|Close_Gate
  (Utilities|FlowControl|Gate false) ; enters at Close
)

(event Custom|Hop
  (Class|Pole|ConductConnection)
  (if (Variables|Default|Getconnected)
    (Utilities|FlowControl|Gate false
      (:Exit
        (CallFunction|Step)))))

(event Custom|OnDataReceptionDelegate_Event_0
  (params (Arr :type Array%20of%20Bytes))
  (bind _returnvalue (Class|Pole|GetAction Arr))
  (Variables|Default|SetActions _returnvalue)
  (CallFunction|OpenGate))