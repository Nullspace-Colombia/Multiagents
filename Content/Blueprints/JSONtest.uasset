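; Test Blueprint that runs a local socket server to exchange agent observations, rewards and actions, apparently for reinforcement learning.
; BeginPlay starts the server and binds the reception delegate; Tick maintains the connection and, once connected, sends hard-coded sample agent data through a Gate.
; The gate closes after each send and reopens when a reply arrives and its agent ID and action are printed, giving lockstep exchange.
; Multi-agent send nodes are present but unwired.
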(event Custom|OnDataReceptionDelegate_Event
  (params (Arr :type Array%20of%20Bytes))
  (Development|PrintString "Received")
  (bind (_agentid _agentaction) (Class|Pole|GetAgentInfo Arr))
  (Development|PrintString _agentid true true "(R=1.000000,G=0.165738,B=0.000000,A=1.000000)" 2e+01)
  (Development|PrintString (Utilities|String|ToString(Float) _agentaction) true true "(R=1.000000,G=0.000000,B=0.962421,A=1.000000)" 2e+01)
  (CallFunction|OpenGate))

(event Custom|Open_Gate
  (Utilities|FlowControl|Gate false) ; enters at Open
)

(event Custom|Close_Gate
  (Utilities|FlowControl|Gate false) ; enters at Close
)

(event EventBeginPlay
  (EventDispatchers|AssignOnDataReceptionDelegate (delegate Custom|OnDataReceptionDelegate_Event))
  (Class|Pole|StartServer "127.0.0.1" 10010))

(event EventTick
  (params (DeltaSeconds :type Float%20%28single-precision%29))
  (Class|Pole|ConductConnection)
  (if (Variables|Default|Getconnected)
    (Utilities|FlowControl|Gate false
      (:Exit
        (Class|Pole|SendAgentInfo (Variables|Default|GetAgentID) (Utilities|Array|MakeArray 1.5 2.36 4.58 -3.25) 1.0 true)
        (Development|PrintString "Sent")
        (CallFunction|CloseGate)))))

(fn ConstructionScript)