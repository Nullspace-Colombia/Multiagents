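; BP_cart is a player-controlled physics cart that is pushed left or right through Enhanced Input.
; On BeginPlay it applies a small one-time rotation to its Cube and adds the IC_cube mapping context for the first player.
; While triggered, the left and right actions apply world Y-axis force to StaticMeshComponent using the Left and Right variables, and print debug strings.
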(event Input|EnhancedActionEvents|EnhancedInputActionIA_cube_left
  (params (ActionValue :type Boolean) (ElapsedSeconds :type Float%20%28double-precision%29) (TriggeredSeconds :type Float%20%28double-precision%29) (InputAction :type Input%20Action%20Object%20Reference :default "/Game/Blueprints/IA_cube_left.IA_cube_left"))
  (:Triggered
    (Development|PrintString "left")
    (Physics|AddForce (Variables|Debug|GetStaticMeshComponent) (Math|Vector|MakeVector 0.0 (Variables|Default|Getleft) 0.0) "None" false)))

(event Input|EnhancedActionEvents|EnhancedInputActionIA_cube_right
  (params (ActionValue :type Boolean) (ElapsedSeconds :type Float%20%28double-precision%29) (TriggeredSeconds :type Float%20%28double-precision%29) (InputAction :type Input%20Action%20Object%20Reference :default "/Game/Blueprints/IA_cube_right.IA_cube_right"))
  (:Triggered
    (Development|PrintString "right")
    (Physics|AddForce (Variables|Debug|GetStaticMeshComponent) (Math|Vector|MakeVector 0.0 (Variables|Default|Getright) 0.0) "None" false)))

(event EventBeginPlay
  (Transformation|AddWorldRotation (Variables|Default|GetCube) "0.000000,0.000000,5.000000" false false)
  (Input|AddMappingContext (PlayerController|LocalPlayerSubsystems|GetEnhancedInputLocalPlayerSubsystem (Game|GetPlayerController 0)) "/Game/Blueprints/IC_cube.IC_cube" 0 "(bIgnoreAllPressedKeysUntilRelease=True,bForceImmediately=False)"))

(fn ConstructionScript)