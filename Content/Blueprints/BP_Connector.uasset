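; Connector that exposes a Cartpole simulation to an external controller as a reinforcement-learning style environment over a localhost socket server.
; Tick services the connection and passes a gate that received data opens, taking the first parsed value as the action.
; Each step checks cart, angle and frame limits, then resets or applies lateral movement with a short delay.
; It sends back state, a counter-based reward and done flag, then closes the gate.
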(event Custom|Step
  (bind _state_info (Variables|Default|GetState_Info))
  (CallFunction|CheckIsDone)
  (if (Variables|Default|GetIsDone)
    (Default|Reset (Variables|Default|GetCartpole))
    (Development|PrintString "\"Resetting\"" true false "(R=1.000000,G=0.812461,B=0.000000,A=1.000000)" 0.8)
    (bind _state (Default|GetState (Variables|Default|GetCartpole) true))
    (for (_array_element _array_index) _state
      (Utilities|Array|SetArrayElem (Variables|Default|GetState_Info) _array_index (Math|Conversions|ToFloat(Integer) _array_element)))
    (Utilities|Array|SetArrayElem (Variables|Default|GetState_Info) 4 (Math|Conversions|ToFloat(Integer) (Variables|Default|GetReward)))
    (Utilities|Array|SetArrayElem (Variables|Default|GetState_Info) 5 (Math|Conversions|ToFloat(Integer) (Math|Conversions|ToFloat(Boolean) (Variables|Default|GetIsDone))))
    (Class|Pole|SendDouble (Variables|Default|GetState_Info))
    (CallFunction|GetReward)
    (for _array_element_2 (Variables|Default|GetState_Info)
      (Development|PrintString (Utilities|String|ToString(Float) _array_element_2)))
    (CallFunction|CloseGate)
    (else
      (Default|AddLateralMovement (Variables|Default|GetCartpole) (Variables|Default|GetAction))
      (Utilities|FlowControl|Delay 0.03)
      (bind _state_2 (Default|GetState (Variables|Default|GetCartpole) true))
      (for (_array_element_3 _array_index_2) _state_2
        (Utilities|Array|SetArrayElem (Variables|Default|GetState_Info) _array_index_2 (Math|Conversions|ToFloat(Integer) _array_element_3)))
      (Utilities|Array|SetArrayElem _state_info 4 (Math|Conversions|ToFloat(Integer) (Variables|Default|GetCounter)))
      (Utilities|Array|SetArrayElem _state_info 5 (Math|Conversions|ToFloat(Integer) (Math|Conversions|ToFloat(Boolean) (Variables|Default|GetIsDone))))
      (Class|Pole|SendDouble (Variables|Default|GetState_Info))
      (CallFunction|GetReward)
      (CallFunction|CloseGate))))

(event Custom|Open_Gate
  (Utilities|FlowControl|Gate false) ; enters at Open
)

(event Custom|Close_Gate
  (Utilities|FlowControl|Gate false) ; enters at Close
)

(event Custom|CheckIsDone
  (bind _state (Default|GetState (Variables|Default|GetCartpole) false))
  (Math|Float|CompareFloat (Math|Float|Absolute(Float) (Utilities|Array|Get(acopy) _state)) (Variables|Default|GetCartPositionThresh)
    (:>
      (Variables|Default|SetIsDone true :!label _label)
      (Variables|Default|SetCounter 0))
    (:==
      (goto _label))
    (:<
      (Math|Float|CompareFloat (Math|Float|Absolute(Float) (Utilities|Array|Get(acopy) _state 2)) (Variables|Default|GetPoleAngleThresh)
        (:>
          (Variables|Default|SetIsDone true :!label _label_2)
          (Variables|Default|SetCounter 0))
        (:==
          (goto _label_2))
        (:<
          (Math|Integer|CompareInt (Variables|Default|GetCounter) (Variables|Default|GetMaxFrames)
            (:>
              (Variables|Default|SetIsDone true :!label _label_3)
              (Variables|Default|SetCounter 0))
            (:==
              (goto _label_3))
            (:<
              (Variables|Default|SetIsDone false))))))))

(event Custom|GetReward
  (bind _result (Math|Integer|IncrementInt (Variables|Default|GetCounter))
    (:%20%20
      (Variables|Default|SetReward _result))))

(event Custom|GetDatatoSend
  (bind _state (Default|GetState (Variables|Default|GetCartpole) true))
  (bind _output_get (Variables|Default|SetState_Info _state))
  (Utilities|Array|Insert _output_get (Math|Conversions|ToFloat(Integer) (Variables|Default|GetReward)))
  (Utilities|Array|Insert (Variables|Default|GetState_Info) (Math|Conversions|ToFloat(Boolean) (Variables|Default|GetIsDone)) 1)
  (for _array_element (Variables|Default|GetState_Info)
    (Development|PrintString (Utilities|String|ToString(Float) _array_element)))
  (Development|PrintString (Utilities|String|ToString(Integer) (Utilities|Array|Length (Variables|Default|GetState_Info)))))

(event Custom|OnDataReceptionDelegate_Event_0
  (params (Arr :type Array%20of%20Bytes))
  (bind _returnvalue (Class|Pole|ParseData Arr))
  (Variables|Default|SetAction (Utilities|Array|Get(acopy) _returnvalue))
  (CallFunction|OpenGate))

(event EventBeginPlay
  (EventDispatchers|AssignOnDataReceptionDelegate (delegate Custom|OnDataReceptionDelegate_Event_0))
  (Class|Pole|StartServer "127.0.0.1" 10010))

(event Collision|EventActorBeginOverlap
  (params (OtherActor :type Actor%20Object%20Reference)))

(event EventTick
  (params (DeltaSeconds :type Float%20%28single-precision%29))
  (Class|Pole|ConductConnection)
  (if (Variables|Default|Getconnected)
    (Utilities|FlowControl|Gate false
      (:Exit
        (CallFunction|Step)))))

(fn ConstructionScript)