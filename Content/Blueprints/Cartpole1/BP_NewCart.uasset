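; Cartpole cart character that serves as a reinforcement learning environment, also drivable by player input.
; Step counts frames and turns a discrete action into left or right movement input, with CharacterMovement set to Flying on BeginPlay.
; GetState reports cart position and velocity plus pole roll and angular velocity; IsDone checks limits and sets the reward.
; Reset spawns and possesses a fresh cart instead of restoring this one, without destroying it here.
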(event Custom|LateralMovement
  (params (NewParam :type Float%20%28double-precision%29))
  (bind _returnvalue (Transformation|GetActorRightVector))
  (if (== NewParam 0.0)
    (Pawn|Input|AddMovementInput _returnvalue 1.0 false)
    (elif (== NewParam 1.0)
      (Pawn|Input|AddMovementInput _returnvalue -1.0 false))))

(event Input|EnhancedActionEvents|EnhancedInputActionIA_MoveLeft
  (params (ActionValue :type Boolean) (ElapsedSeconds :type Float%20%28double-precision%29) (TriggeredSeconds :type Float%20%28double-precision%29) (InputAction :type Input%20Action%20Object%20Reference :default "/Game/Inputs/IA_MoveLeft.IA_MoveLeft"))
  (:Triggered
    (CallFunction|LateralMovement 1.0)
    (CallFunction|GetState)))

(event Input|EnhancedActionEvents|EnhancedInputActionIA_MoveRight
  (params (ActionValue :type Boolean) (ElapsedSeconds :type Float%20%28double-precision%29) (TriggeredSeconds :type Float%20%28double-precision%29) (InputAction :type Input%20Action%20Object%20Reference :default "/Game/Inputs/IA_MoveRight.IA_MoveRight"))
  (:Triggered
    (CallFunction|LateralMovement 0.0)
    (CallFunction|GetState)))

(event EventBeginPlay
  (bind _asplayer_controller (Utilities|Casting|CastToPlayerController (Pawn|GetController)))
  (Utilities|IsValid (PlayerController|LocalPlayerSubsystems|GetEnhancedInputLocalPlayerSubsystem _asplayer_controller)
    (:Is%20Valid
      (Input|AddMappingContext (PlayerController|LocalPlayerSubsystems|GetEnhancedInputLocalPlayerSubsystem _asplayer_controller) "/Game/Inputs/IMC_Cartpole.IMC_Cartpole" 0 "(bIgnoreAllPressedKeysUntilRelease=True,bForceImmediately=False)")
      (Pawn|Components|CharacterMovement|SetMovementMode (Variables|Character|GetCharacterMovement) "MOVE_Flying" 0))))

(event Collision|EventActorBeginOverlap
  (params (OtherActor :type Actor%20Object%20Reference)))

(event EventTick
  (params (DeltaSeconds :type Float%20%28single-precision%29)))

(event EventStep
  (params (Action :type Array%20of%20Floats%20%28double-precision%29))
  (Math|Integer|IncrementInt (Variables|Default|Getcounter)
    (:%20%20
      (CallFunction|LateralMovement (Utilities|Array|Get(acopy) Action)))))

(fn ConstructionScript)

(fn GetID
  (return 0))

(fn GetReward
  (return (Variables|Default|Getreward)))

(fn GetSelfActor
  (return self))

(fn GetState
  (bind _pole (Variables|Default|GetPole))
  (bind _returnvalue (Physics|GetPhysicsLinearVelocity (Variables|Default|GetCart) "None"))
  (return (Utilities|Array|MakeArray (.y (Transformation|GetActorLocation)) (.y _returnvalue) (.roll (Transformation|GetWorldRotation _pole)) (.x (Physics|GetPhysicsAngularVelocityinDegrees _pole "None")))))

(fn IsDone
  (bind _max_cart_position (Variables|Default|Getmax_cart_position))
  (bind _max_pole_angle (Variables|Default|Getmax_pole_angle))
  (bind _observations (CallFunction|GetState))
  (if (Math|Boolean|ANDBoolean (Math|Float|InRange(Float) (Utilities|Array|Get(acopy) _observations) (* _max_cart_position -1.0) _max_cart_position) (Math|Float|InRange(Float) (Utilities|Array|Get(acopy) _observations 2) (* _max_pole_angle -1.0) _max_pole_angle) (<= (Variables|Default|Getcounter) (Variables|Default|Getmax%20frames)))
    (Variables|Default|Setreward 1.0)
    (Variables|Default|Setdone false)
    (else
      (Variables|Default|Setreward 0.0)
      (Variables|Default|Setdone true)))
  (return (Variables|Default|Getdone)))

(fn Reset
  (bind _returnvalue (Transformation|GetActorLocation))
  (bind _returnvalue_2 (Game|SpawnActorfromClass "BP_NewCart_C" (Math|Transform|MakeTransform (Math|Vector|MakeVector (.x _returnvalue) 0.0 (.z _returnvalue)) "0, 0, 0" "1.000000,1.000000,1.000000") "AlwaysSpawn" "MultiplyWithRoot" 0 0))
  (Pawn|Possess (Game|GetPlayerController 0) _returnvalue_2)
  (Variables|Default|Setcounter 0)
  (return _returnvalue_2 true))