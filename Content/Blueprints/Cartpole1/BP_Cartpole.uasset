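; Player-controlled cartpole character that moves sideways, with Cube1's world pitch printed on screen every tick.
; BeginPlay adds the Enhanced Input mapping context, switches CharacterMovement to Flying and applies a one-time velocity-change impulse along world Y.
; IA_Move feeds its X value into movement input along the actor's right vector.
; The Blueprint contains no balancing or control logic, only manual input and the pitch readout.
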(event Input|EnhancedActionEvents|EnhancedInputActionIA_Move
  (params (ActionValue :type Vector%202D%20Structure) (ElapsedSeconds :type Float%20%28double-precision%29) (TriggeredSeconds :type Float%20%28double-precision%29) (InputAction :type Input%20Action%20Object%20Reference :default "/Game/Inputs/IA_Move.IA_Move"))
  (:Triggered
    (Pawn|Input|AddMovementInput (Transformation|GetActorRightVector) (.x ActionValue) false)))

(event EventBeginPlay
  (bind _asplayer_controller (Utilities|Casting|CastToPlayerController (Pawn|GetController)))
  (Utilities|IsValid (PlayerController|LocalPlayerSubsystems|GetEnhancedInputLocalPlayerSubsystem _asplayer_controller)
    (:Is%20Valid
      (Input|AddMappingContext (PlayerController|LocalPlayerSubsystems|GetEnhancedInputLocalPlayerSubsystem _asplayer_controller) "/Game/Inputs/IMC_Cartpole.IMC_Cartpole" 0 "(bIgnoreAllPressedKeysUntilRelease=True,bForceImmediately=False)")
      (Pawn|Components|CharacterMovement|SetMovementMode (Variables|Character|GetCharacterMovement) "MOVE_Flying" 0)
      (Physics|AddImpulse (Variables|Character|GetCharacterMovement) "0.000000,500.000000,0.000000" true))))

(event EventTick
  (params (DeltaSeconds :type Float%20%28single-precision%29))
  (Development|PrintString (Utilities|String|ToString(Float) (.pitch (Transformation|GetWorldRotation (Variables|Default|GetCube1)))) true true "(R=0.318250,G=1.000000,B=0.000000,A=1.000000)" DeltaSeconds))

(fn ConstructionScript)