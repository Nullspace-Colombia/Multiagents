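; BP_Cartpole2D is a two-axis cart-pole environment for reinforcement learning, with a flying-mode pawn as the cart.
; Step actions and Enhanced Input both drive forward/right movement.
; GetState returns pole angles, cart position and velocities; IsDone checks them against thresholds and a frame limit, also setting the reward GetReward returns.
; Reset spawns and possesses a fresh copy rather than restoring the current one.
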(event Custom|AddMovement
  (params (Forward :type Float%20%28double-precision%29) (Right :type Float%20%28double-precision%29))
  ;[0.5697 1 0.4631] Actions
  (Utilities|FlowControl|Sequence
    (:then_0
      (Pawn|Input|AddMovementInput (Transformation|GetActorForwardVector) Forward false))
    (:then_1
      (Pawn|Input|AddMovementInput (Transformation|GetActorRightVector) Right false))))

(event Input|EnhancedActionEvents|EnhancedInputActionIA_Move
  (params (ActionValue :type Vector%202D%20Structure) (ElapsedSeconds :type Float%20%28double-precision%29) (TriggeredSeconds :type Float%20%28double-precision%29) (InputAction :type Input%20Action%20Object%20Reference :default "/Game/Inputs/IA_Move.IA_Move"))
  ;[0.5697 1 0.4631] Actions
  (:Triggered
    (CallFunction|AddMovement (.y ActionValue) (.x ActionValue))))

(event EventBeginPlay
  (bind _asplayer_controller (Utilities|Casting|CastToPlayerController (Pawn|GetController)))
  (Utilities|IsValid (PlayerController|LocalPlayerSubsystems|GetEnhancedInputLocalPlayerSubsystem _asplayer_controller)
    (:Is%20Valid
      (Input|AddMappingContext (PlayerController|LocalPlayerSubsystems|GetEnhancedInputLocalPlayerSubsystem _asplayer_controller) "/Game/Inputs/IMC_Cartpole.IMC_Cartpole" 0 "(bIgnoreAllPressedKeysUntilRelease=True,bForceImmediately=False)")
      (Pawn|Components|CharacterMovement|SetMovementMode (Variables|Character|GetCharacterMovement) "MOVE_Flying" 0))))

(event EventStep
  (params (Action :type Array%20of%20Floats%20%28double-precision%29))
  ;[0.3228 1 0.31] Step
  (Development|PrintString (Utilities|String|Append "Step: " (Utilities|String|ToString(Integer) (Variables|Default|GetCounter))))
  (Math|Integer|IncrementInt (Variables|Default|GetCounter)
    (:%20%20
      (CallFunction|AddMovement (Utilities|Array|Get(acopy) Action) (Utilities|Array|Get(acopy) Action 1)))))

(event EventTick
  (params (DeltaSeconds :type Float%20%28single-precision%29)))

(fn ConstructionScript)

(fn GetState
  (params (PrintState :type Boolean))
  (bind _returnvalue (Transformation|GetActorLocation))
  (bind _cube1 (Variables|Default|GetCube1))
  (bind _stick_base (Variables|Default|Getstick_base))
  (bind _returnvalue_2 (Physics|GetPhysicsAngularVelocityinDegrees _cube1 "None"))
  (bind _returnvalue_3 (Transformation|GetWorldRotation _stick_base))
  (bind _returnvalue_4 (Physics|GetPhysicsLinearVelocity (Variables|Default|GetCube) "None"))
  (return (Utilities|Array|MakeArray (.roll _returnvalue_3) (.pitch _returnvalue_3) (.x _returnvalue) (.y _returnvalue) (.x _returnvalue_2) (.y _returnvalue_2) (.x _returnvalue_4) (.y _returnvalue_4))))

(fn NewFunction)

(fn Reset1
  (bind _returnvalue (Game|SpawnActorfromClass "BP_Cartpole2D_C" (Math|Transform|MakeTransform (Math|Vector|MakeVector 0.0 0.0 (.z (Transformation|GetActorLocation))) "0, 0, 0" "1.000000,1.000000,1.000000") "Undefined" 0 0))
  (Pawn|Possess (Game|GetPlayerController 0) _returnvalue)
  (return _returnvalue))

(fn GetReward
  (return (Math|Conversions|ToFloat(Integer) (Variables|Default|GetReward))))

(fn GetSelfActor
  (return self))

(fn GetState
  (bind _state (CallFunction|GetState false))
  (return _state))

(fn IsDone
  (bind _poleanglethresh_x (Variables|Default|GetPoleAngleThresh_x))
  (bind _poleanglethresh_y (Variables|Default|GetPoleAngleThresh_y))
  (bind _cartpositionthresh_x (Variables|Default|GetCartPositionThresh_x))
  (bind _cartpositionthresh_y (Variables|Default|GetCartPositionThresh_y))
  (bind _state (CallFunction|GetState false))
  (if (Math|Boolean|ANDBoolean (Math|Float|InRange(Float) (Utilities|Array|Get(acopy) _state) (* _poleanglethresh_x -1.0) _poleanglethresh_x) (Math|Float|InRange(Float) (Utilities|Array|Get(acopy) _state 1) (* -1.0 _poleanglethresh_y) _poleanglethresh_y) (Math|Float|InRange(Float) (Utilities|Array|Get(acopy) _state 2) (* _cartpositionthresh_x -1.0) _cartpositionthresh_x) (Math|Float|InRange(Float) (Utilities|Array|Get(acopy) _state 3) (* -1.0 _cartpositionthresh_y) _cartpositionthresh_y))
    (Math|Integer|CompareInt (Variables|Default|GetCounter) (Variables|Default|GetMaxFrames)
      (:>
        (Variables|Default|SetbIsDone true :!label _label)
        (Variables|Default|SetCounter 0)
        (Variables|Default|SetReward 0))
      (:==
        (goto _label))
      (:<
        (Variables|Default|SetbIsDone false)
        (Variables|Default|SetReward 1)))
    (else
      (Variables|Default|SetbIsDone true)
      (Variables|Default|SetCounter 0)
      (Variables|Default|SetReward 0)))
  (return (Variables|Default|GetbIsDone)))

(fn Reset
  (bind _newactor (CallFunction|Reset1))
  (return _newactor true))