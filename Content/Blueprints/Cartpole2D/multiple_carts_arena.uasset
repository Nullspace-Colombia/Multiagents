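; An arena actor that hosts two BP_Cartpole2D agents as child actors.
; On BeginPlay it casts both child actors and stores them as individual references and in an Agents array.
; It then attaches each to the arena root at a fixed relative position, offset along Y, records that position as the agent's InitX and InitY, and resets both.
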(event EventBeginPlay
  (bind _asbp_cartpole_2d (Utilities|Casting|CastToBP_Cartpole2D (Variables|/Script/Engine.ChildActorComponent|GetChildActor (Variables|Default|GetBP_Cartpole2D))))
  (bind _output_get (Variables|Default|SetAgent1 _asbp_cartpole_2d))
  (Utilities|Array|Add (Variables|Default|GetAgents) _output_get)
  (bind _asbp_cartpole_2d_2 (Utilities|Casting|CastToBP_Cartpole2D (Variables|/Script/Engine.ChildActorComponent|GetChildActor (Variables|Default|GetBP_Cartpole2D_agent2))))
  (bind _output_get_2 (Variables|Default|SetAgent2 _asbp_cartpole_2d_2))
  (Utilities|Array|Add (Variables|Default|GetAgents) _output_get_2)
  (Transformation|AttachComponentToComponent (Variables|/Script/Engine.Actor|GetRootComponent _output_get) (Variables|Default|GetDefaultSceneRoot) "None" "KeepRelative" "KeepRelative" "KeepRelative" true)
  (Transformation|SetActorRelativeLocation _output_get "1550.000000,1000.000000,100.000000")
  (Variables|/Game/Blueprints/Cartpole2D/BP_Cartpole2D.BP_Cartpole2D_C|Setinit_x _output_get 1.55e+03)
  (Variables|/Game/Blueprints/Cartpole2D/BP_Cartpole2D.BP_Cartpole2D_C|Setinit_y _output_get 1e+03)
  (Transformation|AttachComponentToComponent (Variables|/Script/Engine.Actor|GetRootComponent _output_get_2) (Variables|Default|GetDefaultSceneRoot) "None" "KeepRelative" "KeepRelative" "KeepRelative" true)
  (Transformation|SetActorRelativeLocation _output_get_2 "1550.000000,1550.000000,100.000000")
  (Variables|/Game/Blueprints/Cartpole2D/BP_Cartpole2D.BP_Cartpole2D_C|Setinit_x _output_get_2 1.55e+03)
  (Variables|/Game/Blueprints/Cartpole2D/BP_Cartpole2D.BP_Cartpole2D_C|Setinit_y _output_get_2 1.55e+03)
  (Default|Reset _output_get_2)
  (Default|Reset _output_get))

(event Collision|EventActorBeginOverlap
  (params (OtherActor :type Actor%20Object%20Reference)))

(event EventTick
  (params (DeltaSeconds :type Float%20%28single-precision%29)))

(fn ConstructionScript)