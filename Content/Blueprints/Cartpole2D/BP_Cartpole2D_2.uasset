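; Cart-pole balancing character that acts as a reinforcement-learning style environment, with Enhanced Input for manual driving in flying movement mode.
; Step counts frames and maps a 0/1 action to backward/forward movement input, so the left key's -1 moves nothing.
; GetState reports cart position and velocity plus pole pitch and angular velocity.
; IsDone checks these against limits and frame cap, setting GetReward's value; Reset spawns a fresh actor.
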(event Custom|AddMovement
  (params (direction :type Float%20%28double-precision%29))
  (bind _returnvalue (Transformation|GetActorForwardVector))
  ;[0.5697 1 0.4631] Actions
  (if (== direction 0.0)
    (Pawn|Input|AddMovementInput _returnvalue -1.0 false)
    (elif (== direction 1.0)
      (Pawn|Input|AddMovementInput _returnvalue 1.0 false))))

(event Input|EnhancedActionEvents|EnhancedInputActionIA_MoveLeft
  (params (ActionValue :type Boolean) (ElapsedSeconds :type Float%20%28double-precision%29) (TriggeredSeconds :type Float%20%28double-precision%29) (InputAction :type Input%20Action%20Object%20Reference :default "/Game/Inputs/IA_MoveLeft.IA_MoveLeft"))
  ;[0.5697 1 0.4631] Actions
  (:Triggered
    (CallFunction|AddMovement -1.0)))

(event Input|EnhancedActionEvents|EnhancedInputActionIA_MoveRight
  (params (ActionValue :type Boolean) (ElapsedSeconds :type Float%20%28double-precision%29) (TriggeredSeconds :type Float%20%28double-precision%29) (InputAction :type Input%20Action%20Object%20Reference :default "/Game/Inputs/IA_MoveRight.IA_MoveRight"))
  ;[0.5697 1 0.4631] Actions
  (:Triggered
    (CallFunction|AddMovement 1.0)))

(event EventBeginPlay
  (bind _asplayer_controller (Utilities|Casting|CastToPlayerController (Pawn|GetController)))
  (Utilities|IsValid (PlayerController|LocalPlayerSubsystems|GetEnhancedInputLocalPlayerSubsystem _asplayer_controller)
    (:Is%20Valid
      (Input|AddMappingContext (PlayerController|LocalPlayerSubsystems|GetEnhancedInputLocalPlayerSubsystem _asplayer_controller) "/Game/Inputs/IMC_Cartpole.IMC_Cartpole" 0 "(bIgnoreAllPressedKeysUntilRelease=True,bForceImmediately=False)")
      (Pawn|Components|CharacterMovement|SetMovementMode (Variables|Character|GetCharacterMovement) "MOVE_Flying" 0))))

(event EventStep
  (params (Action :type Float%20%28double-precision%29))
  ;[0.3228 1 0.31] Step
  (Development|PrintString (Utilities|String|Append "Step: " (Utilities|String|ToString(Integer) (Variables|Default|GetCounter))))
  (Math|Integer|IncrementInt (Variables|Default|GetCounter)
    (:%20%20
      (CallFunction|AddMovement Action))))

(event EventTick
  (params (DeltaSeconds :type Float%20%28single-precision%29)))

(fn ConstructionScript)

(fn GetState
  (bind _returnvalue (Physics|GetPhysicsLinearVelocity (Variables|Default|GetCube) "None"))
  (return (Utilities|Array|MakeArray (.x (Transformation|GetActorLocation)) (.x _returnvalue) (.pitch (Transformation|GetWorldRotation (Variables|Default|Getstick_base))) (.y (Physics|GetPhysicsAngularVelocityinDegrees (Variables|Default|GetCube1) "None")))))

(fn NewFunction)

(fn Reset1)

(fn GetReward
  (return (Math|Conversions|ToFloat(Integer) (Variables|Default|GetReward))))

(fn GetSelfActor
  (return self))

(fn GetState
  (bind _state (CallFunction|GetState))
  (return _state))

(fn IsDone
  (bind _cartpositionthresh_x (Variables|Default|GetCartPositionThresh_x))
  (bind _poleanglethresh_y (Variables|Default|GetPoleAngleThresh_y))
  (bind _state (CallFunction|GetState))
  (if (and (Math|Float|InRange(Float) (Utilities|Array|Get(acopy) _state) (* _cartpositionthresh_x -1.0) _cartpositionthresh_x) (Math|Float|InRange(Float) (Utilities|Array|Get(acopy) _state 2) (* -1.0 _poleanglethresh_y) _poleanglethresh_y))
    (Math|Integer|CompareInt (Variables|Default|GetCounter) (Variables|Default|GetMaxFrames)
      (:>
        (Variables|Default|SetbIsDone true :!label _label)
        (Variables|Default|SetCounter 0)
        (Variables|Default|SetReward 0))
      (:==
        (goto _label))
      (:<
        (Variables|Default|SetbIsDone false)
        (Variables|Default|SetReward 1)))
    (else
      (Variables|Default|SetbIsDone true)
      (Variables|Default|SetCounter 0)
      (Variables|Default|SetReward 0)))
  (return (Variables|Default|GetbIsDone)))

(fn Reset
  (bind _returnvalue (Transformation|GetActorLocation))
  (bind _returnvalue_2 (Game|SpawnActorfromClass "BP_Cartpole2D_2_C" (Math|Transform|MakeTransform (Math|Vector|MakeVector 0.0 (.y _returnvalue) (.z _returnvalue)) "0, 0, 0" "1.000000,1.000000,1.000000") "AlwaysSpawn" "MultiplyWithRoot" 0 0))
  (return _returnvalue_2 true))