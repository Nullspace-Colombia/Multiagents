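; Second agent pawn for a 2D cartpole multi-agent learning environment, a Character in flying mode with the Cartpole input mapping.
; Each Step increments a counter and passes the selected action to the parent's Move; reward, done and state queries also defer to the parent.
; Reset teleports the agent to a fixed spot and repositions the physics-simulated cube by briefly disabling simulation.
; The construction script tints the agent through a dynamic arena material.
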(event Input|EnhancedActionEvents|EnhancedInputActionIA_MoveLeft
  (params (ActionValue :type Boolean) (ElapsedSeconds :type Float%20%28double-precision%29) (TriggeredSeconds :type Float%20%28double-precision%29) (InputAction :type Input%20Action%20Object%20Reference :default "/Game/Inputs/IA_MoveLeft.IA_MoveLeft"))
  ;[0.5697 1 0.4631] Actions
)

(event Input|EnhancedActionEvents|EnhancedInputActionIA_MoveRight
  (params (ActionValue :type Boolean) (ElapsedSeconds :type Float%20%28double-precision%29) (TriggeredSeconds :type Float%20%28double-precision%29) (InputAction :type Input%20Action%20Object%20Reference :default "/Game/Inputs/IA_MoveRight.IA_MoveRight"))
  ;[0.5697 1 0.4631] Actions
)

(event EventBeginPlay
  (bind _asplayer_controller (Utilities|Casting|CastToPlayerController (Pawn|GetController)))
  (Utilities|IsValid (PlayerController|LocalPlayerSubsystems|GetEnhancedInputLocalPlayerSubsystem _asplayer_controller)
    (:Is%20Valid
      (Input|AddMappingContext (PlayerController|LocalPlayerSubsystems|GetEnhancedInputLocalPlayerSubsystem _asplayer_controller) "/Game/Inputs/IMC_Cartpole.IMC_Cartpole" 0 "(bIgnoreAllPressedKeysUntilRelease=True,bForceImmediately=False)")
      (Pawn|Components|CharacterMovement|SetMovementMode (Variables|Character|GetCharacterMovement) "MOVE_Flying" 0))))

(event EventSetID
  (params (ID :type Integer))
  (Variables|Default|SetID ID))

(event EventStep
  (params (Action :type Array%20of%20Floats%20%28double-precision%29))
  ;[0.3228 1 0.31] Step
  (Math|Integer|IncrementInt (Variables|Default|GetCounter)
    (:%20%20
      (CallFunction|Move (Utilities|Array|Get(acopy) Action (Variables|Default|GetAction))))))

(event EventTick
  (params (DeltaSeconds :type Float%20%28single-precision%29)))

(event EventMove
  (params (NewParam :type Float%20%28double-precision%29))
  (|CallParentFunction NewParam))

(event EventSetScenario
  (params (scenario :type Integer)))

(event EventSetActionID
  (params (ActionID :type Integer))
  (Variables|Default|SetAction ActionID))

(fn ConstructionScript
  (bind _returnvalue (Rendering|Material|CreateDynamicMaterialInstance (Variables|Default|GetCube) 0 "/Game/Materials/MultiAgentArena.MultiAgentArena" "None" :!class /Script/Engine.PrimitiveComponent))
  (Rendering|Material|SetVectorParameterValue _returnvalue "Param" (Variables|Default|GetColor) :!class /Script/Engine.MaterialInstanceDynamic))

(fn GetReward
  (bind _reward (|CallParentFunction))
  (return _reward))

(fn IsDone
  (bind _bdone (|CallParentFunction))
  (return _bdone))

(fn Reset
  (bind _cube1 (Variables|Default|GetCube1))
  (Transformation|SetActorLocationAndRotation (Math|Vector|MakeVector 1.55e+03 1.55e+03 (.z (Transformation|GetActorLocation))) "0, 0, 0" false true)
  (Physics|SetSimulatePhysics _cube1 false)
  (Transformation|SetRelativeLocationAndRotation _cube1 "1550.000000,1550.000000,256.000000" "0, 0, 0" false false)
  (Physics|SetSimulatePhysics _cube1 true)
  (return 0 false))

(fn GetState
  (bind _observations (|CallParentFunction))
  (return _observations))

(fn GetSelfActor
  (return self))

(fn GetID
  (return (Variables|Default|GetID)))