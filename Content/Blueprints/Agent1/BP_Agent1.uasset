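; Agent1 character for a two-agent reinforcement learning task with BP_Agent2, also controllable through input actions.
; Step maps an action code to movement, jump or a box grab/drop that attaches BP_Ag_Prop_Box1 to a hand socket.
; GetState returns floor and horizontal ray distances plus location; GetReward scores Y progress minus a time penalty.
; IsDone checks falls, both agents finishing or the frame limit; Reset spawns a replacement and relinks the partner.
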(event OnComponentBeginOverlap(Box)
  (params (OverlappedComponent :type Primitive%20Component%20Object%20Reference) (OtherActor :type Actor%20Object%20Reference) (OtherComp :type Primitive%20Component%20Object%20Reference) (OtherBodyIndex :type Integer) (bFromSweep :type Boolean) (SweepResult :type Hit%20Result%20Structure%20%28by%20ref%29))
  (Utilities|Casting|CastToBP_Ag_Prop_Box1 OtherActor)
  (Variables|Default|SetPush true))

(event OnComponentEndOverlap(Box)
  (params (OverlappedComponent :type Primitive%20Component%20Object%20Reference) (OtherActor :type Actor%20Object%20Reference) (OtherComp :type Primitive%20Component%20Object%20Reference) (OtherBodyIndex :type Integer))
  (Utilities|Casting|CastToBP_Ag_Prop_Box1 OtherActor)
  (Variables|Default|SetPush false))

(event Input|EnhancedActionEvents|EnhancedInputActionIA_MoveDown
  (params (ActionValue :type Boolean) (ElapsedSeconds :type Float%20%28double-precision%29) (TriggeredSeconds :type Float%20%28double-precision%29) (InputAction :type Input%20Action%20Object%20Reference :default "/Game/Inputs/IA_MoveDown.IA_MoveDown"))
  (:Triggered
    (Pawn|Input|AddMovementInput "-1.000000,0.000000,0.000000" 1.0 false)
    (if (> (Math|Vector|VectorLength (Variables|/Script/Engine.MovementComponent|GetVelocity (Variables|Character|GetCharacterMovement))) 0.0)
      (Variables|Default|SetWalk true)
      (else
        (Variables|Default|SetWalk false))))
  (:Completed
    (Variables|Default|SetWalk false)))

(event Input|EnhancedActionEvents|EnhancedInputActionIA_MoveLeft
  (params (ActionValue :type Boolean) (ElapsedSeconds :type Float%20%28double-precision%29) (TriggeredSeconds :type Float%20%28double-precision%29) (InputAction :type Input%20Action%20Object%20Reference :default "/Game/Inputs/IA_MoveLeft.IA_MoveLeft"))
  (:Triggered
    (Pawn|Input|AddMovementInput "0.000000,1.000000,0.000000" -1.0 false)
    (if (> (Math|Vector|VectorLength (Variables|/Script/Engine.MovementComponent|GetVelocity (Variables|Character|GetCharacterMovement))) 0.0)
      (Variables|Default|SetWalk true)
      (else
        (Variables|Default|SetWalk false))))
  (:Completed
    (Variables|Default|SetWalk false)))

(event Input|EnhancedActionEvents|EnhancedInputActionIA_MoveRight
  (params (ActionValue :type Boolean) (ElapsedSeconds :type Float%20%28double-precision%29) (TriggeredSeconds :type Float%20%28double-precision%29) (InputAction :type Input%20Action%20Object%20Reference :default "/Game/Inputs/IA_MoveRight.IA_MoveRight"))
  (:Triggered
    (Pawn|Input|AddMovementInput "0.000000,1.000000,0.000000" 1.0 false)
    (if (> (Math|Vector|VectorLength (Variables|/Script/Engine.MovementComponent|GetVelocity (Variables|Character|GetCharacterMovement))) 0.0)
      (Variables|Default|SetWalk true)
      (else
        (Variables|Default|SetWalk false))))
  (:Completed
    (Variables|Default|SetWalk false)))

(event Input|EnhancedActionEvents|EnhancedInputActionIA_MoveUp
  (params (ActionValue :type Boolean) (ElapsedSeconds :type Float%20%28double-precision%29) (TriggeredSeconds :type Float%20%28double-precision%29) (InputAction :type Input%20Action%20Object%20Reference :default "/Game/Inputs/IA_MoveUp.IA_MoveUp"))
  (:Triggered
    (Pawn|Input|AddMovementInput "1.000000,0.000000,0.000000" 1.0 false)
    (if (> (Math|Vector|VectorLength (Variables|/Script/Engine.MovementComponent|GetVelocity (Variables|Character|GetCharacterMovement))) 0.0)
      (Variables|Default|SetWalk true)
      (else
        (Variables|Default|SetWalk false))))
  (:Completed
    (Variables|Default|SetWalk false)))

(event Input|EnhancedActionEvents|EnhancedInputActionIA_Jump
  (params (ActionValue :type Boolean) (ElapsedSeconds :type Float%20%28double-precision%29) (TriggeredSeconds :type Float%20%28double-precision%29) (InputAction :type Input%20Action%20Object%20Reference :default "/Game/Inputs/IA_Jump.IA_Jump"))
  (:Started
    (Character|Jump)
    (Variables|Default|SetJumping true))
  (:Completed
    (Variables|Default|SetJumping false)))

(event Input|EnhancedActionEvents|EnhancedInputActionIA_Grab
  (params (ActionValue :type Boolean) (ElapsedSeconds :type Float%20%28double-precision%29) (TriggeredSeconds :type Float%20%28double-precision%29) (InputAction :type Input%20Action%20Object%20Reference :default "/Game/Inputs/IA_Grab.IA_Grab"))
  (bind _carrybox (Variables|Default|GetCarryBox))
  (:Completed
    (|AttachBox
      (:true
        (Variables|Default|SetIsCarrying false)
        (Transformation|DetachFromActor _carrybox "KeepWorld" "KeepWorld" "KeepWorld")
        (Physics|SetSimulatePhysics (Variables|/Game/Blueprints/Agent1/BP_Ag_Prop_Box1.BP_Ag_Prop_Box1_C|GetBlueBox _carrybox) true)))))

(event EventBeginPlay
  (bind _returnvalue (Actor|GetActorOfClass "/Game/Blueprints/Agent1/BP_Ag_Prop_Box1.BP_Ag_Prop_Box1_C"))
  (Utilities|IsValid _returnvalue
    (:Is%20Valid
      (Variables|Default|SetCarryBox _returnvalue)
      (bind _returnvalue_2 (Actor|GetActorOfClass "/Game/Blueprints/Agent1/BP_Agent2.BP_Agent2_C"))
      (Variables|Default|SetOther%20agent _returnvalue_2))))

(event Collision|EventActorBeginOverlap
  (params (OtherActor :type Actor%20Object%20Reference)))

(event EventSetActionID
  (params (ActionID :type Integer))
  (Variables|Default|SetAction%20ID ActionID))

(event EventTick
  (params (DeltaSeconds :type Float%20%28single-precision%29))
  (|CollapseGraph)
  (|FloorRay_2_2))

(event EventSetID
  (params (ID :type Integer))
  (Variables|Default|SetID ID))

(event EventStep
  (params (Action :type Array%20of%20Floats%20%28double-precision%29))
  (bind _carrybox (Variables|Default|GetCarryBox))
  (Math|Integer|IncrementInt (Variables|Default|Getcounter)
    (:%20%20
      (bind _action_is_grab_drop (|WASDandJump Action)
        (:out
          (if _action_is_grab_drop
            (if (Utilities|IsValid (Variables|Default|GetCarryBox))
              (|Attach_box
                (:true
                  (Transformation|DetachFromActor _carrybox "KeepRelative" "KeepRelative" "KeepRelative")
                  (Variables|Default|SetIsCarrying false)
                  (Physics|SetSimulatePhysics (Variables|/Game/Blueprints/Agent1/BP_Ag_Prop_Box1.BP_Ag_Prop_Box1_C|GetBlueBox _carrybox) true))))))))))

(fn ConstructionScript)

(fn GetID
  (return 0))

(fn GetReward
  (bind _output_get (Variables|Default|SetReward (- (/ (- (.y (Transformation|GetActorLocation)) (Variables|Default|Getactor%20initial%20position)) (- (Variables|Default|Getfinal%20position) (Variables|Default|Getactor%20initial%20position))) (Variables|Default|Gettime%20penalty))))
  (Development|PrintString (Utilities|String|Append "Reward :  " (Utilities|String|ToString(Float) _output_get)) false false)
  (return (Variables|Default|GetReward)))

(fn GetSelfActor
  (return self))

(fn GetState
  (bind _returnvalue (Transformation|GetActorLocation))
  (bind _total_obs (Variables|Default|GetTotal_obs))
  (Utilities|Array|Clear (Variables|Default|GetTotal_obs))
  (bind _array (|floorrays))
  (Utilities|Array|AppendArray (Variables|Default|GetTotal_obs) _array)
  (bind _array_2 (|upperbodyrays))
  (Utilities|Array|AppendArray _total_obs _array_2)
  (Utilities|Array|AppendArray _total_obs (Utilities|Array|MakeArray (.x _returnvalue) (.y _returnvalue) (.z _returnvalue)))
  (Development|PrintString (Utilities|String|ToString(Float) (.z _returnvalue)) false false)
  (return (Variables|Default|GetTotal_obs)))

(fn IsDone
  (bind _returnvalue (Transformation|GetActorLocation))
  (bind _other_agent (Variables|Default|GetOther%20agent))
  (bind _returnvalue_2 (Transformation|GetActorLocation _other_agent))
  (bind _output_get (Variables|Default|Setdone (Math|Boolean|ORBoolean (<= (.z _returnvalue) 0.0) (and (>= (.y _returnvalue) 4.83e+03) (>= (.y _returnvalue_2) 4.83e+03)) (<= (.z _returnvalue_2) 0.0) (>= (Variables|Default|Getcounter) (Variables|Default|GetMax%20frames)))))
  (return _output_get))

(fn Reset
  (Variables|Default|Setcounter 0)
  (bind _returnvalue (Game|SpawnActorfromClass "BP_Agent1_C" (Math|Transform|MakeTransform "0.000000,-99.000000,88.000000" "0, 0, 0" "1.000000,1.000000,1.000000") "AlwaysSpawn" "MultiplyWithRoot" 0 0))
  (bind _returnvalue_2 (Actor|GetActorOfClass "/Game/Blueprints/Agent1/BP_Agent2.BP_Agent2_C"))
  (Variables|Default|SetOther%20agent _returnvalue_2)
  (Variables|BP_Agent1_C|SetOther%20agent (Variables|Default|GetOther%20agent) _returnvalue)
  (Variables|Default|Setdone false)
  (Development|PrintString "reset")
  (return _returnvalue true))