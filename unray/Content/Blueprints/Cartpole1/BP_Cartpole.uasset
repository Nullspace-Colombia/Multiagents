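; BP_Cartpole is a cart-pole character serving as a reinforcement-learning environment, with Step, GetState, GetReward, IsDone and Reset functions.
; Agent actions and Enhanced Input both push the cart left or right through movement input in flying mode.
; State comprises cart position, cart velocity, pole roll and angular velocity; position, angle or frame limits end episodes and zero the reward.
; Reset spawns and possesses a fresh copy rather than repositioning the current one.
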(event Custom|AddLateralMovement
  (params (Input :type Float%20%28double-precision%29))
  ;[0.5697 1 0.4631] Actions
  (if (== Input 0.0)
    (Pawn|Input|AddMovementInput (Transformation|GetActorRightVector) -1.0 false)
    (elif (== Input 1.0)
      (Pawn|Input|AddMovementInput (Transformation|GetActorRightVector) 1.0 false))))

(event Input|EnhancedActionEvents|EnhancedInputActionIA_MoveLeft
  (params (ActionValue :type Boolean) (ElapsedSeconds :type Float%20%28double-precision%29) (TriggeredSeconds :type Float%20%28double-precision%29) (InputAction :type Input%20Action%20Object%20Reference :default "/unray/Inputs/IA_MoveLeft.IA_MoveLeft"))
  ;[0.5697 1 0.4631] Actions
  (:Triggered
    (CallFunction|AddLateralMovement 0.0)))

(event Input|EnhancedActionEvents|EnhancedInputActionIA_MoveRight
  (params (ActionValue :type Boolean) (ElapsedSeconds :type Float%20%28double-precision%29) (TriggeredSeconds :type Float%20%28double-precision%29) (InputAction :type Input%20Action%20Object%20Reference :default "/unray/Inputs/IA_MoveRight.IA_MoveRight"))
  ;[0.5697 1 0.4631] Actions
  (:Triggered
    (CallFunction|AddLateralMovement 1.0)))

(event EventBeginPlay
  (bind _asplayer_controller (Utilities|Casting|CastToPlayerController (Pawn|GetController)))
  (Utilities|IsValid (PlayerController|LocalPlayerSubsystems|GetEnhancedInputLocalPlayerSubsystem _asplayer_controller)
    (:Is%20Valid
      (Input|AddMappingContext (PlayerController|LocalPlayerSubsystems|GetEnhancedInputLocalPlayerSubsystem _asplayer_controller) "/unray/Inputs/IMC_Cartpole.IMC_Cartpole" 0 "(bIgnoreAllPressedKeysUntilRelease=True,bForceImmediately=False)")
      (Pawn|Components|CharacterMovement|SetMovementMode (Variables|Character|GetCharacterMovement) "MOVE_Flying" 0))))

(event EventStep
  (params (Action :type Array%20of%20Floats%20%28double-precision%29))
  ;[0.3228 1 0.31] Step
  (Development|PrintString (Utilities|String|Append "Step: " (Utilities|String|ToString(Integer) (Variables|Default|GetCounter))) true false)
  (Math|Integer|IncrementInt (Variables|Default|GetCounter)
    (:%20%20
      (CallFunction|AddLateralMovement (Utilities|Array|Get(acopy) Action)))))

(event EventTick
  (params (DeltaSeconds :type Float%20%28single-precision%29)))

(fn ConstructionScript)

(fn GetState
  (params (PrintState :type Boolean))
  (bind _returnvalue (Transformation|GetActorLocation))
  (bind _cube1 (Variables|Default|GetCube1))
  (bind _scene (Variables|Default|GetScene))
  (bind _returnvalue_2 (Physics|GetPhysicsAngularVelocityinDegrees _cube1 "None"))
  (bind _returnvalue_3 (Transformation|GetWorldRotation _scene))
  (if PrintState
    (Development|PrintString (Utilities|String|ToString(Float) (.roll _returnvalue_3)) true false "(R=0.318250,G=1.000000,B=0.000000,A=1.000000)" (Utilities|Time|GetWorldDeltaSeconds))
    (Development|PrintString (Utilities|String|ToString(Float) (.y _returnvalue)) true false "(R=0.000000,G=0.660000,B=1.000000,A=1.000000)" (Utilities|Time|GetWorldDeltaSeconds))
    (Development|PrintString (Utilities|String|ToString(Float) (.x _returnvalue_2)) true false "(R=1.000000,G=0.653868,B=0.000000,A=1.000000)" (Utilities|Time|GetWorldDeltaSeconds))
    (bind _returnvalue_4 (Physics|GetPhysicsLinearVelocity (Variables|Default|GetCube) "None"))
    (Development|PrintString (Utilities|String|ToString(Float) (.y _returnvalue_4)) true false "(R=0.966027,G=0.562004,B=1.000000,A=1.000000)" (Utilities|Time|GetWorldDeltaSeconds))
    (else
      (bind _returnvalue_5 (Physics|GetPhysicsLinearVelocity (Variables|Default|GetCube) "None"))))
  (return (Utilities|Array|MakeArray (.y _returnvalue) (.y _returnvalue_5) (.roll _returnvalue_3) (.x _returnvalue_2))))

(fn Reset1
  (bind _returnvalue (Transformation|GetActorLocation))
  (bind _returnvalue_2 (Game|SpawnActorfromClass "BP_Cartpole_C" (Math|Transform|MakeTransform (Math|Vector|MakeVector (.x _returnvalue) 0.0 (.z _returnvalue)) "0, 0, 0" "1.000000,1.000000,1.000000") "Undefined" 0 0))
  (Pawn|Possess (Game|GetPlayerController 0) _returnvalue_2)
  (return _returnvalue_2))

(fn GetID
  (return 0))

(fn GetReward
  (return (Math|Conversions|ToFloat(Integer) (Variables|Default|GetReward))))

(fn GetSelfActor
  (return self))

(fn GetState
  (bind _state (CallFunction|GetState false))
  (return _state))

(fn IsDone
  (bind _state (CallFunction|GetState false))
  (Math|Float|CompareFloat (Math|Float|Absolute(Float) (Utilities|Array|Get(acopy) _state)) (Variables|Default|GetCartPositionThresh)
    (:>
      (Variables|Default|SetbIsDone true :!label _label)
      (Variables|Default|SetCounter 0)
      (Variables|Default|SetReward 0))
    (:==
      (goto _label))
    (:<
      (Math|Float|CompareFloat (Math|Float|Absolute(Float) (Utilities|Array|Get(acopy) _state 2)) (Variables|Default|GetPoleAngleThresh)
        (:>
          (Variables|Default|SetbIsDone true :!label _label_2)
          (Variables|Default|SetCounter 0)
          (Variables|Default|SetReward 0))
        (:==
          (goto _label_2))
        (:<
          (Math|Integer|CompareInt (Variables|Default|GetCounter) (Variables|Default|GetMaxFrames)
            (:>
              (Variables|Default|SetbIsDone true :!label _label_3)
              (Variables|Default|SetCounter 0)
              (Variables|Default|SetReward 0))
            (:==
              (goto _label_3))
            (:<
              (Variables|Default|SetbIsDone false)
              (Variables|Default|SetReward 1)))))))
  (return (Variables|Default|GetbIsDone)))

(fn Reset
  (bind _new_actor (CallFunction|Reset1))
  (return _new_actor true))